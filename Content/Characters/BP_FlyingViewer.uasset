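; BP_FlyingViewer is a pawn or character that views from the air before diving into the battle.
; Turn and LookUp axes drive controller yaw and pitch, and the Interaction input asks BP_BattlePC to dive through WantToDive.
; On remote instances, BeginPlay sets the widget component's interaction prompt to "하강" (descend).
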(event `self.ReceiveBeginPlay`
  (`/Engine/EditorBlueprintResources/ActorMacros.Switch Has Authority`
    (:`Remote`
      (bind _aswidget_bp_interaction (cast `/Game/Characters/HUD/WidgetBP_Interaction` (`WidgetComponent.GetUserWidgetObject` (`self.Widget`))))
      (set `/Game/Characters/HUD/WidgetBP_Interaction.InteractionText` "하강" _aswidget_bp_interaction))))

(event `InputAxis|Turn`
  (params (AxisValue :type "Float (single-precision)"))
  (`self.AddControllerYawInput` AxisValue))

(event `InputAxis|LookUp`
  (params (AxisValue :type "Float (single-precision)"))
  (`self.AddControllerPitchInput` AxisValue))

(event `InputAction|Interaction`
  (params (Key :type "Key Structure"))
  (:`Pressed`
    (bind _asbp_battle_pc (cast `/Game/GameModes/Battle/BP_BattlePC` (`self.GetController`)))
    (`/Game/GameModes/Battle/BP_BattlePC.WantToDive` _asbp_battle_pc)))

(fn `UserConstructionScript`)