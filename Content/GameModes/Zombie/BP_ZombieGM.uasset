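; Game mode for a two-player zombie wave-defense match around a Nexus, with a boss in wave ten.
; A one-second looping timer drives the waiting, battle, intermission, ceremony and defeat states, using zombie count to end waves.
; Waves spawns escalating normal and upgraded zombies at four locations.
; It respawns dead players with saved gear and stats, and relays messages, Nexus/boss HP and results to player controllers.
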(event `self.K2_PostLogin`
  (params (NewPlayer :type "PlayerController Object Reference"))
  ;[1 1 1] PostLogin/Out
  (bind _asbp_zombie_pc (cast `/Game/GameModes/Zombie/BP_ZombiePC` NewPlayer))
  (if (`|EnumEquality` (`self.PlayingState`) "NewEnumerator0")
    (`KismetArrayLibrary.Array_Add` (`self.AlivePCs`) _asbp_zombie_pc)
    (set `self.PlayerNum` (+ (`self.PlayerNum`) 1))
    (set `/Game/GameModes/Zombie/BP_ZombiePC.NotificationFromServer` "어서오세요. 환영합니다." _asbp_zombie_pc)
    (else
      (`self.SetLifeSpan` 0.1))))

(event `self.K2_OnLogout`
  (params (ExitingController :type "Controller Object Reference"))
  ;[1 1 1] PostLogin/Out
  (bind _asbp_zombie_pc (cast `/Game/GameModes/Zombie/BP_ZombiePC` ExitingController))
  (`KismetArrayLibrary.Array_RemoveItem` (`self.AlivePCs`) _asbp_zombie_pc)
  (set `self.PlayerNum` (- (`self.PlayerNum`) 1)))

(event `SpawnMainTaget`
  ;[1 1 1] Main
  (bind _returnvalue (`|SpawnActorFromClass` "/Game/Nexus/BP_Nexus.BP_Nexus_C" (`KismetMathLibrary.Conv_VectorToTransform` (`self.TargetLocation`)) "Undefined" "OverrideRootScale" null null))
  (set `self.MainTarget` _returnvalue))

(event `self.ReceiveBeginPlay`
  (set `self.RemainTimeToStart` (`self.WaitingTime`))
  (bind _returnvalue (`KismetSystemLibrary.K2_SetTimerDelegate` (delegate `MainTimer`) 1.0 true))
  (set `self.MainTimerHandle` _returnvalue))

(event `MainTimer`
  (bind _remaintimetostart (`self.RemainTimeToStart`))
  (bind _remaintimetostart_2 (`self.RemainTimeToStart`))
  (`self.Timer`)
  (switch `/Game/GameModes/Battle/EPlayingState` (`self.PlayingState`)
    (:`NewEnumerator0`
      (if (== (`self.PlayerNum`) 2)
        (bind _result (`/Engine/EditorBlueprintResources/StandardMacros.DecrementInt` _remaintimetostart)
          (:`  `
            (if (== _result 0)
              (`|ExecutionSequence`
                (:`then_0`
                  (set `self.WaveNum` 1)
                  (`self.ReturnWaveNum`)
                  (set `self.IsTimerON` true))
                (:`then_1`
                  (`self.SayToAll` (`KismetTextLibrary.Conv_TextToString` (`|FormatText` "Wave{T} Start" (`self.WaveNum`)))))
                (:`then_2`
                  (`KismetSystemLibrary.Delay` 3.0)
                  (`self.SayToAll` ""))
                (:`then_3`
                  (for _array_element (`self.AlivePCs`)
                    (`/Engine/EditorBlueprintResources/StandardMacros.IsValid` _array_element
                      (:`Is Valid`
                        (`/Game/GameModes/Zombie/BP_ZombiePC.PlayInit` _array_element)
                        (`/Game/GameModes/Zombie/BP_ZombiePC.PlayBGM` _array_element)))))
                (:`then_4`
                  (`self.SpawnMainTaget`)
                  (`self.CreateEnemySpawner`))
                (:`then_5`
                  (`self.Waves` (`self.WaveNum`))
                  (set `self.PlayingState` "NewEnumerator1")
                  (`self.PlayZombieSound`)))
              (else
                (`self.SayToAll` (`KismetTextLibrary.Conv_TextToString` (`|FormatText` "전투시작까지 {T} 남았습니다." (`self.FormatMinSec` _remaintimetostart))))))))
        (else
          (set `self.RemainTimeToStart` (`self.WaitingTime`))
          (`self.SayToAll` "다른 유저의 접속을 기다리는 중 입니다."))))
    (:`NewEnumerator1`
      (if (== (`self.RealDeath`) 2)
        _
        (elif (`self.Defeat`)
          _
          (elif (<= (`self.NumOfZombie`) 0)
            (set `self.RemainTimeToStart` 10)
            (set `self.PlayingState` "NewEnumerator4")
            (else
              (set `self.PlayingState` "NewEnumerator1"))))))
    (:`NewEnumerator4`
      (if (`self.IsWin`)
        (set `self.PlayingState` "NewEnumerator2")
        (else
          (bind _result_2 (`/Engine/EditorBlueprintResources/StandardMacros.DecrementInt` _remaintimetostart_2)
            (:`  `
              (if (== _result_2 0)
                (bind _output_get (set `self.WaveNum` (+ (`self.WaveNum`) 1)))
                (`self.ReturnWaveNum`)
                (`self.Waves` _output_get)
                (`self.PlayZombieSound`)
                (`self.SayToAll` "")
                (set `self.PlayingState` "NewEnumerator1")
                (else
                  (`self.SayToAll` (`KismetTextLibrary.Conv_TextToString` (`|FormatText` "다음 웨이브까지 {T} 남았습니다." (`self.FormatMinSec` _remaintimetostart_2)))))))))))
    (:`NewEnumerator2`
      (`/Engine/EditorBlueprintResources/StandardMacros.DoOnce` false
        (:`Completed`
          (`self.ShowResult_WIN`)
          (set `self.IsTimerON` false :!label _label))))
    (:`NewEnumerator3`
      (`/Engine/EditorBlueprintResources/StandardMacros.DoOnce` false
        (:`Completed`
          (`self.ShowResult_DEFEAT`)
          (goto _label))))))

(event `CreateEnemySpawner`
  (bind _returnvalue (`|SpawnActorFromClass` "/Game/Enemy/EnemySpawner/BP_EnemySpawner.BP_EnemySpawner_C" (`KismetMathLibrary.Conv_VectorToTransform` (`self.EnemySpawnerLocation`)) "Undefined" "OverrideRootScale" self null))
  (set `self.EnemySpawner` _returnvalue))

(event `Spawner_Spawn`
  (params (`타겟` :type "/Game/Enemy/EnemySpawner/BP_EnemySpawner Object Reference") (Enemy :type "Actor Class Reference") (SpawnTransform :type "Transform Structure") (`Num Of Enemies` :type Integer) (SpawnDelay :type "Float (double-precision)") (MaxSpawn :type Integer))
  (`/Game/Enemy/EnemySpawner/BP_EnemySpawner.SpawnEnemy` `타겟` Enemy SpawnTransform `Num Of Enemies` SpawnDelay MaxSpawn))

(event `FunctionDelay`
  (params (Duration :type "Float (double-precision)"))
  (`KismetSystemLibrary.Delay` Duration))

(event `IncreaseZombie`
  (set `self.NumOfZombie` (+ (`self.NumOfZombie`) 1)))

(event `Timer`
  (bind _sec (`self.Sec`))
  (if (`self.IsTimerON`)
    (set `self.Sec` (+ _sec 1))
    (if (== _sec 60)
      (set `self.Sec` 0)
      (set `self.Min` (+ (`self.Min`) 1)))))

(event `DecreaseZombie`
  (set `self.NumOfZombie` (- (`self.NumOfZombie`) 1)))

(event `SetDefeat`
  (params (Defeat :type Boolean))
  (set `self.Defeat` Defeat))

(event `SpawnZombie1`
  (params (LastIndex :type Integer) (UpgradeZombie :type Boolean))
  ;[1 1 1] SpawnZombie
  (for _ (range 1 (+ LastIndex 1))
    (bind _returnvalue (`|SpawnActorFromClass` "/Game/Enemy/Zombie/BP_ZombieDefault.BP_ZombieDefault_C" (`KismetMathLibrary.Conv_VectorToTransform` (`self.SpawnLocation1`)) "AdjustIfPossibleButAlwaysSpawn" "OverrideRootScale" null null))
    (if UpgradeZombie
      (`/Game/Enemy/Zombie/BP_ZombieDefault.UpgradeZombie` _returnvalue))))

(event `OnCharacterDeath`
  (params (PC :type "/Game/GameModes/Zombie/BP_ZombiePC Object Reference"))
  (bind _deadpcs (`self.DeadPCs`))
  (bind _output (`|GetArrayItem` _deadpcs))
  (`KismetArrayLibrary.Array_Add` _deadpcs PC)
  (bind _asbp_player_base (cast `/Game/Characters/BP_PlayerBase` (`Controller.K2_GetPawn` _output)))
  (set `self.HelmetLevel` (`/Game/Characters/BP_PlayerBase.HelmetLevel` _asbp_player_base))
  (set `self.UpperLevel` (`/Game/Characters/BP_PlayerBase.UpperLevel` _asbp_player_base))
  (set `self.LowerLevel` (`/Game/Characters/BP_PlayerBase.LowerLevel` _asbp_player_base))
  (set `self.ShoesLevel` (`/Game/Characters/BP_PlayerBase.ShoesLevel` _asbp_player_base))
  (set `self.WeaponID` (`/Game/Characters/BP_PlayerBase.WeaponItemClassID` _asbp_player_base))
  (set `self.Dollar` (`/Game/Characters/BP_PlayerBase.Dollar` _asbp_player_base))
  (set `self.Kill` (`/Game/Characters/BP_PlayerBase.ZombieKillNum` _asbp_player_base))
  (set `self.Death` (`/Game/Characters/BP_PlayerBase.DeathNum` _asbp_player_base))
  (set `self.DamageRifle` (`/Game/Characters/BP_PlayerBase.Damage_Rifle` _asbp_player_base))
  (set `self.DamageShotgun` (`/Game/Characters/BP_PlayerBase.Damage_Shotgun` _asbp_player_base))
  (set `self.Armor` (`/Game/Characters/BP_PlayerBase.Armor` _asbp_player_base))
  (set `/Game/GameModes/Zombie/BP_ZombiePC.RespawnMessage` "죽었습니다! 잠시후 부활합니다." _output)
  (`KismetSystemLibrary.Delay` 5.0)
  (set `/Game/GameModes/Zombie/BP_ZombiePC.RespawnMessage` "" _output)
  (`self.SpawnPlayer` (`KismetMathLibrary.Conv_VectorToTransform` (`self.PlayerRespawnLocation`))))

(event `SpawnZombie2`
  (params (LastIndex :type Integer) (UpgradeZombie :type Boolean))
  ;[1 1 1] SpawnZombie
  (for _ (range 1 (+ LastIndex 1))
    (bind _returnvalue (`|SpawnActorFromClass` "/Game/Enemy/Zombie/BP_ZombieDefault.BP_ZombieDefault_C" (`KismetMathLibrary.Conv_VectorToTransform` (`self.SpawnLocation2`)) "AdjustIfPossibleButAlwaysSpawn" "OverrideRootScale" null null))
    (if UpgradeZombie
      (`/Game/Enemy/Zombie/BP_ZombieDefault.UpgradeZombie` _returnvalue))))

(event `SpawnZombie3`
  (params (LastIndex :type Integer) (UpgradeZombie :type Boolean))
  ;[1 1 1] SpawnZombie
  (for _ (range 1 (+ LastIndex 1))
    (bind _returnvalue (`|SpawnActorFromClass` "/Game/Enemy/Zombie/BP_ZombieDefault.BP_ZombieDefault_C" (`KismetMathLibrary.Conv_VectorToTransform` (`self.SpawnLocation3`)) "AdjustIfPossibleButAlwaysSpawn" "OverrideRootScale" null null))
    (if UpgradeZombie
      (`/Game/Enemy/Zombie/BP_ZombieDefault.UpgradeZombie` _returnvalue))))

(event `SpawnZombie4`
  (params (LastIndex :type Integer) (UpgradeZombie :type Boolean))
  ;[1 1 1] SpawnZombie
  (for _ (range 1 (+ LastIndex 1))
    (bind _returnvalue (`|SpawnActorFromClass` "/Game/Enemy/Zombie/BP_ZombieDefault.BP_ZombieDefault_C" (`KismetMathLibrary.Conv_VectorToTransform` (`self.SpawnLocation4`)) "AdjustIfPossibleButAlwaysSpawn" "OverrideRootScale" null null))
    (if UpgradeZombie
      (`/Game/Enemy/Zombie/BP_ZombieDefault.UpgradeZombie` _returnvalue))))

(event `SpawnBoss`
  ;[1 1 1] SpawnZombie
  (`KismetSystemLibrary.Delay` 2.0)
  (`|SpawnActorFromClass` "/Game/Enemy/Boss/BP_Boss.BP_Boss_C" (`KismetMathLibrary.Conv_VectorToTransform` (`self.EnemySpawnerLocation`)) "AdjustIfPossibleButAlwaysSpawn" "OverrideRootScale" null null))

(event `SpawnPlayer`
  (params (SpawnTransform :type "Transform Structure"))
  (if (== (`self.PlayerDeathCount`) 6)
    (set `self.RealDeath` (+ (`self.RealDeath`) 1))
    (else
      (bind _returnvalue (`|SpawnActorFromClass` "/Game/Characters/BP_PlayerBase.BP_PlayerBase_C" SpawnTransform "AdjustIfPossibleButAlwaysSpawn" "OverrideRootScale" (`|GetArrayItem` (`self.DeadPCs`)) null))
      (`Controller.Possess` (`|GetArrayItem` (`self.DeadPCs`)) _returnvalue)
      (`KismetArrayLibrary.Array_Remove` (`self.DeadPCs`))
      (`|ExecutionSequence`
        (:`then_0`
          (`/Game/Characters/BP_PlayerBase.UpgradeHelmet_Req` _returnvalue (`self.HelmetLevel`)))
        (:`then_1`
          (`/Game/Characters/BP_PlayerBase.UpgradeUpper_Req` _returnvalue (`self.UpperLevel`)))
        (:`then_2`
          (`/Game/Characters/BP_PlayerBase.UpgradeLower_Req` _returnvalue (`self.LowerLevel`)))
        (:`then_3`
          (`/Game/Characters/BP_PlayerBase.UpgradeShoes_Req` _returnvalue (`self.ShoesLevel`)))
        (:`then_4`
          (`/Game/Characters/BP_PlayerBase.ChangeWeaponByShop` _returnvalue (`self.WeaponID`)))
        (:`then_5`
          (`/Game/Characters/BP_PlayerBase.ChangeDollar` _returnvalue (`self.Dollar`)))
        (:`then_6`
          (`/Game/Characters/BP_PlayerBase.ChangeInfo` _returnvalue (`self.Kill`) (`self.Death`) (`self.DamageRifle`) (`self.DamageShotgun`) (`self.Armor`)))))))

(fn `FormatMinSec`
  (params (Sec :type Integer))
  (returns (TimeText :type Text))
  (locals (Text :type String))
  (bind _returnvalue (/ Sec 60))
  (bind _returnvalue_2 (mod Sec 60))
  (if (not (== _returnvalue 0))
    (set `local.Text` (`KismetStringLibrary.Concat_StrStr` (`KismetStringLibrary.Conv_IntToString` _returnvalue) "분 ")))
  (if (not (== _returnvalue_2 0))
    (bind _output_get (set `local.Text` (`KismetStringLibrary.Concat_StrStr` (`local.Text`) (`KismetStringLibrary.Conv_IntToString` _returnvalue_2) "초"))))
  (return (`KismetTextLibrary.Conv_StringToText` _output_get)))

(fn `PlayZombieSound`
  (for _array_element (`self.AlivePCs`)
    (`/Engine/EditorBlueprintResources/StandardMacros.IsValid` _array_element
      (:`Is Valid`
        (`/Game/GameModes/Zombie/BP_ZombiePC.PlayWaveStart` _array_element)))))

(fn `ReturnWaveNum`
  (for _array_element (`self.AlivePCs`)
    (`/Game/GameModes/Zombie/BP_ZombiePC.GetResultInfo` _array_element (`self.WaveNum`) 0 0 "" false)))

(fn `SayToAll`
  (params (Message :type String))
  (`|ExecutionSequence`
    (:`then_0`
      (for _array_element (`self.AlivePCs`)
        (`/Engine/EditorBlueprintResources/StandardMacros.IsValid` _array_element
          (:`Is Valid`
            (set `/Game/GameModes/Zombie/BP_ZombiePC.NotificationFromServer` Message _array_element)))))
    (:`then_1`
      (for _array_element_2 (`self.DeadPCs`)
        (`/Engine/EditorBlueprintResources/StandardMacros.IsValid` _array_element_2
          (:`Is Valid`
            (set `/Game/GameModes/Zombie/BP_ZombiePC.NotificationFromServer` Message _array_element_2)))))))

(fn `ShowResult_DEFEAT`
  (`|ExecutionSequence`
    (:`then_0`
      (for _array_element (`self.AlivePCs`)
        (`/Engine/EditorBlueprintResources/StandardMacros.IsValid` _array_element
          (:`Is Valid`
            (`/Game/GameModes/Zombie/BP_ZombiePC.GetResultInfo` _array_element (`self.WaveNum`) (`self.Sec`) (`self.Min`) "DEFEAT" true)))))
    (:`then_1`
      (for _array_element_2 (`self.DeadPCs`)
        (`/Engine/EditorBlueprintResources/StandardMacros.IsValid` _array_element_2
          (:`Is Valid`
            (`/Game/GameModes/Zombie/BP_ZombiePC.GetResultInfo` _array_element_2 (`self.WaveNum`) (`self.Sec`) (`self.Min`) "DEFEAT" true)))))))

(fn `ShowResult_WIN`
  (`|ExecutionSequence`
    (:`then_0`
      (for _array_element (`self.AlivePCs`)
        (`/Engine/EditorBlueprintResources/StandardMacros.IsValid` _array_element
          (:`Is Valid`
            (`/Game/GameModes/Zombie/BP_ZombiePC.GetResultInfo` _array_element (`self.WaveNum`) (`self.Sec`) (`self.Min`) "WIN" true)))))
    (:`then_1`
      (for _array_element_2 (`self.DeadPCs`)
        (`/Engine/EditorBlueprintResources/StandardMacros.IsValid` _array_element_2
          (:`Is Valid`
            (`/Game/GameModes/Zombie/BP_ZombiePC.GetResultInfo` _array_element_2 (`self.WaveNum`) (`self.Sec`) (`self.Min`) "WIN" true)))))))

(fn `UpdateBossHP`
  (params (BossHP :type "Float (double-precision)"))
  (`|ExecutionSequence`
    (:`then_0`
      (for _array_element (`self.AlivePCs`)
        (`/Engine/EditorBlueprintResources/StandardMacros.IsValid` _array_element
          (:`Is Valid`
            (set `/Game/GameModes/Zombie/BP_ZombiePC.BossHP` BossHP _array_element)))))
    (:`then_1`
      (for _array_element_2 (`self.DeadPCs`)
        (`/Engine/EditorBlueprintResources/StandardMacros.IsValid` _array_element_2
          (:`Is Valid`
            (set `/Game/GameModes/Zombie/BP_ZombiePC.BossHP` BossHP _array_element_2)))))))

(fn `UpdateNexusHP`
  (params (NexusHP :type "Float (double-precision)"))
  (`|ExecutionSequence`
    (:`then_0`
      (for _array_element (`self.AlivePCs`)
        (`/Engine/EditorBlueprintResources/StandardMacros.IsValid` _array_element
          (:`Is Valid`
            (bind _output_get (set `/Game/GameModes/Zombie/BP_ZombiePC.NexusHP` NexusHP _array_element))
            (set `self.NexusHP` _output_get)
            (if (<= (`self.NexusHP`) 0.0) :!label _label
              (set `self.PlayingState` "NewEnumerator3"))))))
    (:`then_1`
      (for _array_element_2 (`self.DeadPCs`)
        (`/Engine/EditorBlueprintResources/StandardMacros.IsValid` _array_element_2
          (:`Is Valid`
            (bind _output_get_2 (set `/Game/GameModes/Zombie/BP_ZombiePC.NexusHP` NexusHP _array_element_2))
            (set `self.NexusHP` _output_get_2)
            (goto _label)))))))

(fn `UserConstructionScript`)

(fn `Waves`
  (params (WaveNum :type Integer))
  (if (== WaveNum 1)
    (`self.SpawnZombie1` 5)
    (`self.SpawnZombie4` 5)
    (elif (== WaveNum 2)
      (`self.SpawnZombie1` 5)
      (`self.SpawnZombie2` 5)
      (`self.SpawnZombie4` 5)
      (elif (== WaveNum 3)
        (`self.SpawnZombie1` 5)
        (`self.SpawnZombie2` 5)
        (`self.SpawnZombie3` 5)
        (`self.SpawnZombie4` 5)
        (elif (== WaveNum 4)
          (`self.SpawnZombie1` 6)
          (`self.SpawnZombie2` 6)
          (`self.SpawnZombie3` 6)
          (`self.SpawnZombie4` 6)
          (elif (== WaveNum 5)
            (`self.SpawnZombie1` 7)
            (`self.SpawnZombie2` 7)
            (`self.SpawnZombie3` 7)
            (`self.SpawnZombie4` 7)
            (elif (== WaveNum 6)
              (`self.SpawnZombie1` 8)
              (`self.SpawnZombie2` 8)
              (`self.SpawnZombie3` 7)
              (`self.SpawnZombie4` 7 true)
              (elif (== WaveNum 7)
                (`self.SpawnZombie1` 8)
                (`self.SpawnZombie2` 8)
                (`self.SpawnZombie3` 7 true)
                (`self.SpawnZombie4` 7 true)
                (elif (== WaveNum 8)
                  (`self.SpawnZombie1` 8)
                  (`self.SpawnZombie2` 8 true)
                  (`self.SpawnZombie3` 8 true)
                  (`self.SpawnZombie4` 8 true)
                  (elif (== WaveNum 9)
                    (`self.SpawnZombie1` 9 true)
                    (`self.SpawnZombie2` 8 true)
                    (`self.SpawnZombie3` 8 true)
                    (`self.SpawnZombie4` 8 true)
                    (elif (== WaveNum 10)
                      (`self.SpawnZombie1` 9 true)
                      (`self.SpawnZombie2` 9 true)
                      (`self.SpawnZombie3` 9 true)
                      (`self.SpawnZombie4` 8 true)
                      (`self.SpawnBoss`))))))))))))