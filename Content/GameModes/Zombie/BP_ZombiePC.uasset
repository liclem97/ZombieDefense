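; Player controller for the zombie wave mode, managing each player's UI, input mode, sounds and links to BP_ZombieGM.
; BeginPlay creates the main HUD only without authority, while key input opens the Tab and shop widgets.
; Zombie count changes, deaths and respawns forward to the game mode, and events toggle blood, reload and boss overlays.
; Tick watches IsGameEnd and, once, shows the result screen from stored match info and pawn stats.
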(event `InputAction|Tab`
  (params (Key :type "Key Structure"))
  (:`Pressed`
    (`/Engine/EditorBlueprintResources/StandardMacros.IsValid` (`self.WidgetBP_Tab`)
      (:`Is Valid`
        (`Widget.SetVisibility` (`self.WidgetBP_Tab`) "Visible"))
      (:`Is Not Valid`
        (bind _returnvalue (`|CreateWidget` "/Game/Characters/HUD/WidgetBP_Tab.WidgetBP_Tab_C" self (`self.WaveNum`) self))
        (bind _output_get (set `self.WidgetBP_Tab` _returnvalue))
        (`UserWidget.AddToViewport` _output_get 0))))
  (:`Released`
    (`Widget.SetVisibility` (`self.WidgetBP_Tab`) "Hidden")))

(event `InputAction|Shop`
  (params (Key :type "Key Structure"))
  (:`Pressed`
    (bind _asbp_player_base (cast `/Game/Characters/BP_PlayerBase` (`self.K2_GetPawn`)))
    (if (not (`/Game/Characters/BP_PlayerBase.IsShopOpen` _asbp_player_base))
      (`/Engine/EditorBlueprintResources/StandardMacros.IsValid` (`self.WidgetBP_Shop`)
        (:`Is Valid`
          _)
        (:`Is Not Valid`
          (bind _returnvalue (`|CreateWidget` "/Game/Characters/HUD/WidgetBP_Shop.WidgetBP_Shop_C" self self))
          (set `self.WidgetBP_Shop` _returnvalue)))
      (`UserWidget.AddToViewport` (`self.WidgetBP_Shop`) 0)
      (bind _asbp_player_base_2 (cast `/Game/Characters/BP_PlayerBase` (`self.K2_GetPawn`)))
      (set `/Game/Characters/BP_PlayerBase.IsShopOpen` true _asbp_player_base_2)
      (`WidgetBlueprintLibrary.SetInputMode_UIOnlyEx` self (`self.WidgetBP_Shop`))
      (set `self.bShowMouseCursor` true)
      (`Widget.SetVisibility` (`self.WidgetBP_Main`) "Hidden"))))

(event `IncreaseZombie`
  (set `self.NumOfZombies` (+ (`self.NumOfZombies`) 1))
  (`/Game/GameModes/Zombie/BP_ZombieGM.IncreaseZombie` (`self.GameMode`)))

(event `GetResultInfo`
  (params (WaveNum :type Integer) (Sec :type Integer) (Min :type Integer) (ResultString :type String) (IsGameEnd :type Boolean))
  (`|ExecutionSequence`
    (:`then_0`
      (set `self.WaveNum` WaveNum))
    (:`then_1`
      (set `self.Sec` Sec))
    (:`then_2`
      (set `self.Min` Min))
    (:`then_3`
      (set `self.ResultString` ResultString))
    (:`then_4`
      (set `self.IsGameEnd` IsGameEnd))))

(event `self.ReceiveBeginPlay`
  (`WidgetBlueprintLibrary.SetInputMode_GameOnly` self)
  (set `self.bShowMouseCursor` false)
  (`|ExecutionSequence`
    (:`then_0`
      (`/Engine/EditorBlueprintResources/ActorMacros.Switch Has Authority`
        (:`Remote`
          (bind _asbp_zombie_gs (cast `/Game/GameModes/Zombie/BP_ZombieGS` (`GameplayStatics.GetGameState`)))
          (bind _returnvalue (`|CreateWidget` "/Game/Characters/HUD/WidgetBP_Main.WidgetBP_Main_C" self self _asbp_zombie_gs))
          (bind _output_get (set `self.WidgetBP_Main` _returnvalue))
          (`UserWidget.AddToViewport` _output_get 0))))
    (:`then_1`
      (bind _asbp_zombie_gm (cast `/Game/GameModes/Zombie/BP_ZombieGM` (`GameplayStatics.GetGameMode`)))
      (set `self.GameMode` _asbp_zombie_gm))))

(event `DecreaseZombie`
  (set `self.NumOfZombies` (- (`self.NumOfZombies`) 1))
  (`/Game/GameModes/Zombie/BP_ZombieGM.DecreaseZombie` (`self.GameMode`)))

(event `PlayBGM`
  ;[1 1 1] Sound
  (`GameplayStatics.PlaySound2D` "/Game/Sound/Tenebrous.Tenebrous"))

(event `PlayWaveStart`
  ;[1 1 1] Sound
  (`GameplayStatics.PlaySound2D` "/Game/Sound/zombie-15965.zombie-15965"))

(event `self.ReceiveTick`
  (params (DeltaSeconds :type "Float (single-precision)"))
  (if (`self.IsGameEnd`)
    (`/Engine/EditorBlueprintResources/StandardMacros.DoOnce` false
      (:`Completed`
        (`self.ShowResult` (`self.ResultString`) (`self.WaveNum`) (`self.Min`) (`self.Sec`))))))

(event `ShowResult`
  (params (ResultMessage :type String) (WaveMessage :type Integer) (MinMessage :type Integer) (SecMessage :type Integer))
  (bind _asbp_player_base (cast `/Game/Characters/BP_PlayerBase` (`self.K2_GetPawn`)))
  (bind _returnvalue (`|CreateWidget` "/Game/Characters/HUD/WidgetBP_Result.WidgetBP_Result_C" self ResultMessage WaveMessage MinMessage SecMessage (`/Game/Characters/BP_PlayerBase.ZombieKillNum` _asbp_player_base) (`/Game/Characters/BP_PlayerBase.DeathNum` _asbp_player_base) (`/Game/Characters/BP_PlayerBase.HelmetLevel` _asbp_player_base) (`/Game/Characters/BP_PlayerBase.UpperLevel` _asbp_player_base) (`/Game/Characters/BP_PlayerBase.LowerLevel` _asbp_player_base) (`/Game/Characters/BP_PlayerBase.ShoesLevel` _asbp_player_base) (`/Game/Characters/BP_PlayerBase.AttackUpNum` _asbp_player_base)))
  (`UserWidget.AddToViewport` _returnvalue 0)
  (`WidgetBlueprintLibrary.SetInputMode_UIOnlyEx` self)
  (set `self.bShowMouseCursor` true)
  (`Widget.RemoveFromParent` (`self.WidgetBP_Main`)))

(event `PlaySoundLose`
  ;[1 1 1] Sound
  (`GameplayStatics.PlaySound2D` "/Game/Sound/Tenebrous.Tenebrous"))

(event `PlayBloodAnim`
  (bind _widgetbp_main (`self.WidgetBP_Main`))
  (`Widget.SetVisibility` (`/Game/Characters/HUD/WidgetBP_Main.Blood` _widgetbp_main) "Visible")
  (`UserWidget.PlayAnimation` _widgetbp_main (`/Game/Characters/HUD/WidgetBP_Main.BloodAnimation` _widgetbp_main) 0.0 0 "Forward" 1.0))

(event `PlayInit`
  (bind _asbp_player_base (cast `/Game/Characters/BP_PlayerBase` (`self.K2_GetPawn`)))
  (set `/Game/Characters/BP_PlayerBase.Dollar` 1500 _asbp_player_base))

(event `OnCharacterDeath`
  (bind _returnvalue (`GameplayStatics.GetGameMode`))
  (`/Engine/EditorBlueprintResources/StandardMacros.IsValid` _returnvalue
    (:`Is Valid`
      (bind _asbp_zombie_gm (cast `/Game/GameModes/Zombie/BP_ZombieGM` _returnvalue))
      (`/Game/GameModes/Zombie/BP_ZombieGM.OnCharacterDeath` _asbp_zombie_gm self))))

(event `StopBloodAnim`
  (bind _widgetbp_main (`self.WidgetBP_Main`))
  (bind _blood (`/Game/Characters/HUD/WidgetBP_Main.Blood` _widgetbp_main))
  (`/Engine/EditorBlueprintResources/StandardMacros.IsValid` _blood
    (:`Is Valid`
      (`Widget.SetVisibility` _blood "Hidden")
      (`UserWidget.StopAnimation` _widgetbp_main (`/Game/Characters/HUD/WidgetBP_Main.BloodAnimation` _widgetbp_main)))))

(event `PlayerResurrection`
  (bind _returnvalue (`GameplayStatics.GetGameMode`))
  (`/Engine/EditorBlueprintResources/StandardMacros.IsValid` _returnvalue
    (:`Is Valid`
      (bind _asbp_zombie_gm (cast `/Game/GameModes/Zombie/BP_ZombieGM` _returnvalue)
        (:`then`
          (`KismetSystemLibrary.PrintString` "cast success")
          (`/Game/GameModes/Zombie/BP_ZombieGM.SpawnPlayer` _asbp_zombie_gm (`KismetMathLibrary.Conv_VectorToTransform` (`self.GetActorForwardVector` (`GameplayStatics.GetPlayerCharacter` 0)))))
        (:`CastFailed`
          (`KismetSystemLibrary.PrintString` "cast failed"))))
    (:`Is Not Valid`
      (`KismetSystemLibrary.PrintString` "gameMode not valid"))))

(event `ShowBossUI`
  (`Widget.SetVisibility` (`/Game/Characters/HUD/WidgetBP_Main.Overlay_Boss` (`self.WidgetBP_Main`)) "Visible"))

(event `SetReloadText`
  (params (IsReload :type Boolean))
  (bind _overlay_reload (`/Game/Characters/HUD/WidgetBP_Main.Overlay_Reload` (`self.WidgetBP_Main`)))
  (if IsReload
    (`Widget.SetVisibility` _overlay_reload "Visible")
    (else
      (`Widget.SetVisibility` _overlay_reload "Hidden"))))

(event `UpdateKill`
  (params (Kill :type Integer))
  ;[1 1 1] Update
  (set `self.Kill` Kill))

(event `UpdateArmor`
  (params (ArmorLV :type Integer))
  ;[1 1 1] Update
  (set `self.ArmorLV` ArmorLV))

(event `UpdateDeath`
  (params (Death :type Integer))
  ;[1 1 1] Update
  (set `self.Death` Death))

(event `UpdatePants`
  (params (PantsLV :type Integer))
  ;[1 1 1] Update
  (set `self.PantsLV` PantsLV))

(event `UpdateHelmet`
  (params (HelmetLV :type Integer))
  ;[1 1 1] Update
  (set `self.HelmetLV` HelmetLV))

(event `UpdateShoes`
  (params (ShoesLV :type Integer))
  ;[1 1 1] Update
  (set `self.ShoesLV` ShoesLV))

(event `UpdateAttack`
  (params (AttackUp :type Integer))
  ;[1 1 1] Update
  (set `self.AttackUp` AttackUp))

(fn `UserConstructionScript`)