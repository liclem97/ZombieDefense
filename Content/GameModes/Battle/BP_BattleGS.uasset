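; Battle game state that runs the phased, battle-royale style shrinking electric field.
; Each phase loads from EletricFieldPhaseTable by number, optionally randomizing the next target around the previous circle, and precomputes per-second position and radius deltas.
; UpdateCircle_MainTimer, not started here, counts down wait, show and shrink stages, toggles circle visibility, steps the circle, then advances the phase.
; Stage announcements broadcast through BP_BattleGM and clear after a delay.
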(event `Notify`
  (params (Message :type String))
  (bind _asbp_battle_gm (cast `/Game/GameModes/Battle/BP_BattleGM` (`GameplayStatics.GetGameMode`)))
  (`/Game/GameModes/Battle/BP_BattleGM.SayToAll` _asbp_battle_gm Message)
  (`KismetSystemLibrary.K2_SetTimerDelegate` (delegate `ResetMessage`) 5.0))

(event `ResetMessage`
  (bind _asbp_battle_gm (cast `/Game/GameModes/Battle/BP_BattleGM` (`GameplayStatics.GetGameMode`)))
  (`/Game/GameModes/Battle/BP_BattleGM.SayToAll` _asbp_battle_gm ""))

(event `UpdateCircle_MainTimer`
  (bind _result (`/Engine/EditorBlueprintResources/StandardMacros.DecrementInt` (`self.WaitingTime`))
    (:`  `
      (if (not (>= _result 0))
        (if (not (`self.VisibleTargetCircle`))
          (set `self.VisibleTargetCircle` true))
        (bind _result_2 (`/Engine/EditorBlueprintResources/StandardMacros.DecrementInt` (`self.ShowTime`))
          (:`  `
            (if (>= _result_2 0)
              (if (not (`self.NotifiedShowTime`))
                (`self.Notify` "새로운 자기장 영역이 설정되었습니다.")
                (set `self.NotifiedShowTime` true))
              (else
                (if (not (`self.VisibleCurrentCircle`))
                  (set `self.VisibleCurrentCircle` true))
                (bind _result_3 (`/Engine/EditorBlueprintResources/StandardMacros.DecrementInt` (`self.ShrinkTime`))
                  (:`  `
                    (if (>= _result_3 0)
                      (set `self.CurrentCirclePosition` (+ (`self.CurrentCirclePosition`) (`self.DeltaPositionPerSec`)))
                      (set `self.CurrentCircleRadius` (+ (`self.CurrentCircleRadius`) (`self.DeltaRadiusPerSec`)))
                      (if (not (`self.NotifiedShrinkTime`))
                        (`self.Notify` "자기장 영역이 줄어들기 시작합니다.")
                        (set `self.NotifiedShrinkTime` true))
                      (elif (`self.VisibleTargetCircle`)
                        (set `self.VisibleTargetCircle` false)
                        (`self.SetEletricFieldPhase` (+ (`self.CurrentPhase`) 1) (`self.TargetCirclePosition`) (`self.TargetCircleRadius`))))))))))))))

(event `self.ReceiveBeginPlay`
  (`self.SetEletricFieldPhase` 1))

(event `SetEletricFieldPhase`
  (params (Phase :type Integer) (PreviousCirclePosition :type "Vector Structure") (PreviousCircleRadius :type "Float (double-precision)"))
  (set `self.NotifiedShowTime` false)
  (set `self.NotifiedShrinkTime` false)
  (bind _returnvalue (`|GetDataTableRow` "/Game/GameModes/Battle/EletricFieldPhaseTable.EletricFieldPhaseTable" (`KismetStringLibrary.Conv_StringToName` (`KismetStringLibrary.Conv_IntToString` Phase)))
    (:`then`
      (set `self.CurrentPhase` (break `/Game/GameModes/Battle/EletricFieldPhase` _returnvalue))
      (set `self.CurrentCirclePosition` (`.CurrentCirclePosition_5_059DE55C42AF33010D632EB8164A6CFE` (break `/Game/GameModes/Battle/EletricFieldPhase` _returnvalue)))
      (set `self.CurrentCircleRadius` (`.CurrentCircleRadius_8_F8B408494E1D96BE49EA809F499C714C` (break `/Game/GameModes/Battle/EletricFieldPhase` _returnvalue)))
      (set `self.TargetCirclePosition` (`.TargetCirclePosition_11_2566144E434F2A7E5377498B84A7D791` (break `/Game/GameModes/Battle/EletricFieldPhase` _returnvalue)))
      (set `self.TargetCircleRadius` (`.TargetCircleRadius_14_33EFD591414553D052FCF580D8C2E922` (break `/Game/GameModes/Battle/EletricFieldPhase` _returnvalue)))
      (set `self.WaitingTime` (`.WaitTime_17_2361A2284AFA7B62A9119CADED180D31` (break `/Game/GameModes/Battle/EletricFieldPhase` _returnvalue)))
      (set `self.ShowTime` (`.ShowTime_19_8A5763A749238A7EA723F5BEE2B12C55` (break `/Game/GameModes/Battle/EletricFieldPhase` _returnvalue)))
      (set `self.ShrinkTime` (`.ShrinkTime_21_F490BAD343AAD735A482E58507C9AD85` (break `/Game/GameModes/Battle/EletricFieldPhase` _returnvalue)))
      (set `self.VisibleCurrentCircle` false)
      (if (> (`self.CurrentPhase`) 1)
        (set `self.VisibleCurrentCircle` true))
      (set `self.VisibleTargetCircle` false)
      (if (`.UseRandomTarget_26_0D4D612A4E9DF1F9FF2C01A08F7599DE` (break `/Game/GameModes/Battle/EletricFieldPhase` _returnvalue))
        (bind _output_get (set `self.CurrentCirclePosition` PreviousCirclePosition))
        (set `self.CurrentCircleRadius` PreviousCircleRadius)
        (set `self.TargetCirclePosition` (+ _output_get (* (`KismetMathLibrary.RandomUnitVector`) (`KismetMathLibrary.RandomFloatInRange` (`.RandomTargetDistanceMin_31_B71E23AE4994C04B88AD4F8C867BF82F` (break `/Game/GameModes/Battle/EletricFieldPhase` _returnvalue)) (`.RandomTargetDistanceMax_32_D29EE1834F60E915C615BD8D2DBF07BB` (break `/Game/GameModes/Battle/EletricFieldPhase` _returnvalue)))))))
      (set `self.DeltaPositionPerSec` (/ (- (`self.TargetCirclePosition`) (`self.CurrentCirclePosition`)) (`self.ShrinkTime`)))
      (set `self.DeltaRadiusPerSec` (/ (- (`self.TargetCircleRadius`) (`self.CurrentCircleRadius`)) (`KismetMathLibrary.Conv_IntToDouble` (`self.ShrinkTime`)))))))

(fn `UserConstructionScript`)