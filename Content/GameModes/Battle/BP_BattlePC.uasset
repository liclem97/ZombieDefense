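; BP_BattlePC is the battle-mode player controller, taking the player from riding a C130 plane to diving as a character.
; It swaps pawns by possessing a flying viewer attached to the plane, then spawning a diving BP_PlayerBase below it once.
; It creates the client HUD, toggles the world map, supplies pawn position and heading, and forwards deaths to BP_BattleGM.
; Death and winner result events are empty stubs.
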(event `RideInC130`
  (params (C130 :type "/Game/Vehicles/C-130/BP_C130 Object Reference"))
  (`self.K2_DestroyActor` (`self.K2_GetPawn`))
  (`self.UnPossess`)
  (bind _returnvalue (`|SpawnActorFromClass` "/Game/Characters/BP_FlyingViewer.BP_FlyingViewer_C" (`self.GetTransform` C130) "AlwaysSpawn" "OverrideRootScale" self null))
  (`self.Possess` _returnvalue)
  (`self.K2_AttachToActor` _returnvalue C130 "None" "SnapToTarget" "SnapToTarget" "SnapToTarget" false))

(event `self.ReceiveBeginPlay`
  (`|ExecutionSequence`
    (:`then_0`
      (bind _outactors (`GameplayStatics.GetAllActorsWithTag` "C130"))
      (if (> (`KismetArrayLibrary.Array_Length` _outactors) 0)
        (bind _asbp_c130 (cast `/Game/Vehicles/C-130/BP_C130` (`|GetArrayItem` _outactors)))
        (set `self.C130` _asbp_c130)
        (`WidgetBlueprintLibrary.SetInputMode_GameOnly` self)
        (set `self.bShowMouseCursor` false)
        (`/Engine/EditorBlueprintResources/ActorMacros.Switch Has Authority`
          (:`Remote`
            (bind _asbp_battle_gs (cast `/Game/GameModes/Battle/BP_BattleGS` (`GameplayStatics.GetGameState`)))
            (bind _returnvalue (`|CreateWidget` "/Game/GameModes/Battle/UMG/WidgetBP_ClientMain.WidgetBP_ClientMain_C" self self _asbp_battle_gs))
            (bind _output_get (set `self.WidgetBP_ClientMain` _returnvalue))
            (`UserWidget.AddToViewport` _output_get 0)))))))

(event `ShowBloodScreenEffect`
  (bind _widgetbp_clientmain (`self.WidgetBP_ClientMain`))
  (`/Engine/EditorBlueprintResources/StandardMacros.IsValid` _widgetbp_clientmain
    (:`Is Valid`
      (`UserWidget.PlayAnimation` _widgetbp_clientmain (`/Game/GameModes/Battle/UMG/WidgetBP_ClientMain.BloodScreenEffect` _widgetbp_clientmain) 0.0 1 "Forward" 1.0))))

(event `OnCharacterDeath`
  (bind _returnvalue (`GameplayStatics.GetGameMode`))
  (`/Engine/EditorBlueprintResources/StandardMacros.IsValid` _returnvalue
    (:`Is Valid`
      (bind _asbp_battle_gm (cast `/Game/GameModes/Battle/BP_BattleGM` _returnvalue))
      (`/Game/GameModes/Battle/BP_BattleGM.OnCharacterDeath` _asbp_battle_gm self))))

(event `ShowDeathResult`
  (params (Rank :type Integer)))

(event `ShowWinnerResult`)

(event `BackToLobby`
  (`GameplayStatics.OpenLevel` "Lobby"))

(event `WantToDive`
  (if (not (`self.Dived`))
    (set `self.Dived` true)
    (bind _returnvalue (`|SpawnActorFromClass` "/Game/Characters/BP_PlayerBase.BP_PlayerBase_C" (`KismetMathLibrary.MakeTransform` (`KismetMathLibrary.MakeVector` (.x (`self.K2_GetActorLocation` (`self.K2_GetPawn`))) (.y (`self.K2_GetActorLocation` (`self.K2_GetPawn`))) (- (.z (`self.K2_GetActorLocation` (`self.K2_GetPawn`))) 1000.0))) "AlwaysSpawn" "OverrideRootScale" self null))
    (`self.K2_DestroyActor` (`self.K2_GetPawn`))
    (`self.Possess` _returnvalue)
    (set `/Game/Characters/BP_PlayerBase.Diving` true _returnvalue)))

(event `InputAction|Worldmap`
  (params (Key :type "Key Structure"))
  (bind _widgetbp_worldmap (`self.WidgetBP_Worldmap`))
  (:`Pressed`
    (`/Engine/EditorBlueprintResources/StandardMacros.FlipFlop`
      (:`A`
        (`/Engine/EditorBlueprintResources/StandardMacros.IsValid` (`self.WidgetBP_Worldmap`)
          (:`Is Valid`
            (`UserWidget.AddToViewport` (`self.WidgetBP_Worldmap`) 0))
          (:`Is Not Valid`
            (bind _returnvalue (`|CreateWidget` "/Game/Worldmap/WidgetBP_Worldmap.WidgetBP_Worldmap_C" self self))
            (bind _output_get (set `self.WidgetBP_Worldmap` _returnvalue))
            (`UserWidget.AddToViewport` _output_get 0))))
      (:`B`
        (`/Engine/EditorBlueprintResources/StandardMacros.IsValid` _widgetbp_worldmap
          (:`Is Valid`
            (`Widget.RemoveFromParent` _widgetbp_worldmap)))))))

(fn `GetPawnPosition`
  (returns (PawnPosition :type "Vector Structure") (MapSize :type "Vector Structure") (Airplane :type Boolean) (Forward :type "Vector Structure"))
  (locals (Airplane_ :type Boolean) (Forward_ :type "Vector Structure"))
  (bind _returnvalue (`self.K2_GetPawn`))
  (`/Engine/EditorBlueprintResources/StandardMacros.IsValid` _returnvalue
    (:`Is Valid`
      (cast `/Game/Characters/BP_FlyingViewer` _returnvalue
        (:`then`
          (set `local.Airplane_` true)
          (set `local.Forward_` (`self.GetActorForwardVector` (`self.C130`))))
        (:`CastFailed`
          (set `local.Airplane_` false)
          (set `local.Forward_` (`self.GetActorForwardVector` _returnvalue))))
      (return (`self.K2_GetActorLocation` _returnvalue) (`self.MapSize`) (`local.Airplane_`) (`local.Forward_`)))
    (:`Is Not Valid`
      (return (999999986991104.0 1.0000000272564224e+16 0.0) (`self.MapSize`) (`local.Airplane_`) (`local.Forward_`)))))

(fn `UserConstructionScript`)