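; Game mode for a battle-royale match, driven by a one-second timer through Waiting, Battle and Ceremony states.
; Waiting counts down once enough players join, then enables damage and loads everyone into the C130; late joiners are removed.
; Battle updates the GameState circle and alive count until one remains; its out-of-circle check has no effect yet.
; Ceremony counts down, returns players to lobby and reopens the level as listen server.
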(event `self.K2_PostLogin`
  (params (NewPlayer :type "PlayerController Object Reference"))
  (bind _asbp_battle_pc (cast `/Game/GameModes/Battle/BP_BattlePC` NewPlayer))
  (if (`|EnumEquality` (`self.PlayingState`) "NewEnumerator0")
    (`KismetArrayLibrary.Array_Add` (`self.AlivePCs`) _asbp_battle_pc)
    (set `/Game/GameModes/Battle/BP_BattlePC.NotificationFromServer` "어서오세요. 환영합니다." _asbp_battle_pc)
    (else
      (`self.SetLifeSpan` _asbp_battle_pc 0.1))))

(event `self.K2_OnLogout`
  (params (ExitingController :type "Controller Object Reference"))
  (bind _asbp_battle_pc (cast `/Game/GameModes/Battle/BP_BattlePC` ExitingController))
  (`KismetArrayLibrary.Array_RemoveItem` (`self.AlivePCs`) _asbp_battle_pc))

(event `self.ReceiveBeginPlay`
  (set `self.RemainTimeToStart` (`self.WaitingTime`))
  (bind _outactors (`GameplayStatics.GetAllActorsWithTag` "C130"))
  (if (> (`KismetArrayLibrary.Array_Length` _outactors) 0)
    (bind _asbp_c130 (cast `/Game/Vehicles/C-130/BP_C130` (`|GetArrayItem` _outactors))
      (:`then`
        (set `self.C130` _asbp_c130)
        (bind _returnvalue (`KismetSystemLibrary.K2_SetTimerDelegate` (delegate `MainTimer`) 1.0 true))
        (set `self.MainTimerHandle` _returnvalue))
      (:`CastFailed`
        (`KismetSystemLibrary.PrintString` "C130 Not Found" true true (struct :`G` 0.66 :`B` 1.0 :`A` 1.0) 30.0 :!label _label)))
    (else
      (goto _label))))

(event `MainTimer`
  (bind _alivepcs (`self.AlivePCs`))
  (bind _remaintimetostart (`self.RemainTimeToStart`))
  (switch `/Game/GameModes/Battle/EPlayingState` (`self.PlayingState`)
    (:`NewEnumerator0`
      (if (>= (`KismetArrayLibrary.Array_Length` (`self.AlivePCs`)) (`self.MinimumPlayerCount`))
        (bind _result (`/Engine/EditorBlueprintResources/StandardMacros.DecrementInt` _remaintimetostart)
          (:`  `
            (if (== _result 0)
              (`|ExecutionSequence`
                (:`then_0`
                  (set `self.PlayingState` "NewEnumerator1"))
                (:`then_1`
                  (bind _asbp_battle_gs (cast `/Game/GameModes/Battle/BP_BattleGS` (`GameplayStatics.GetGameState`)))
                  (set `/Game/GameModes/Battle/BP_BattleGS.DamageAvailable` true _asbp_battle_gs))
                (:`then_2`
                  (`self.SayToAll` "전투를 시작합니다."))
                (:`then_3`
                  (for _array_element (`self.AlivePCs`)
                    (`/Engine/EditorBlueprintResources/StandardMacros.IsValid` _array_element
                      (:`Is Valid`
                        (`/Game/GameModes/Battle/BP_BattlePC.RideInC130` _array_element (`self.C130`))))))
                (:`then_4`
                  (set `/Game/Vehicles/C-130/BP_C130.Started` true (`self.C130`)))
                (:`then_5`
                  (`KismetSystemLibrary.Delay` 5.0)
                  (`self.SayToAll` "")))
              (else
                (`self.SayToAll` (`KismetTextLibrary.Conv_TextToString` (`|FormatText` "전투시작까지 {T} 남았습니다." (`self.FormatMinSec` _remaintimetostart))))))))
        (else
          (set `self.RemainTimeToStart` (`self.WaitingTime`))
          (`self.SayToAll` "다른 유저의 접속을 기다리는 중 입니다."))))
    (:`NewEnumerator1`
      (bind _asbp_battle_gs_2 (cast `/Game/GameModes/Battle/BP_BattleGS` (`GameplayStatics.GetGameState`)))
      (`/Game/GameModes/Battle/BP_BattleGS.UpdateCircle_MainTimer` _asbp_battle_gs_2)
      (bind _output_get (set `/Game/GameModes/Battle/BP_BattleGS.AliveCount` (`KismetArrayLibrary.Array_Length` _alivepcs) _asbp_battle_gs_2))
      (if (<= _output_get 1)
        (`/Game/GameModes/Battle/BP_BattlePC.ShowWinnerResult` (`|GetArrayItem` _alivepcs))
        (set `self.PlayingState` "NewEnumerator2")
        (else
          (`|ExecutionSequence`
            (:`then_0`
              (bind _asbp_battle_gs_3 (cast `/Game/GameModes/Battle/BP_BattleGS` (`GameplayStatics.GetGameState`)))
              (if (`/Game/GameModes/Battle/BP_BattleGS.VisibleCurrentCircle` _asbp_battle_gs_3)
                (for _array_element_2 (`self.AlivePCs`)
                  (bind _asbp_player_base (cast `/Game/Characters/BP_PlayerBase` (`Controller.K2_GetPawn` _array_element_2)))
                  (if (>= (`KismetMathLibrary.VSize` (- (`KismetMathLibrary.MakeVector` (.x (`self.K2_GetActorLocation` _asbp_player_base)) (.y (`self.K2_GetActorLocation` _asbp_player_base))) (`KismetMathLibrary.MakeVector` (.x (`/Game/GameModes/Battle/BP_BattleGS.CurrentCirclePosition` _asbp_battle_gs_3)) (.y (`/Game/GameModes/Battle/BP_BattleGS.CurrentCirclePosition` _asbp_battle_gs_3))))) (`/Game/GameModes/Battle/BP_BattleGS.CurrentCircleRadius` _asbp_battle_gs_3))
                    _))))))))
    (:`NewEnumerator2`
      (bind _result_2 (`/Engine/EditorBlueprintResources/StandardMacros.DecrementInt` (`self.RemainTimeOfCeremony`))
        (:`  `
          (if (== _result_2 0)
            (`KismetSystemLibrary.K2_ClearAndInvalidateTimerHandle` (`self.MainTimerHandle`))
            (`|ExecutionSequence`
              (:`then_0`
                (for _array_element_3 (`self.AlivePCs`)
                  (`/Engine/EditorBlueprintResources/StandardMacros.IsValid` _array_element_3
                    (:`Is Valid`
                      (`/Game/GameModes/Battle/BP_BattlePC.BackToLobby` _array_element_3)))))
              (:`then_1`
                (for _array_element_4 (`self.DeadPCs`)
                  (`/Engine/EditorBlueprintResources/StandardMacros.IsValid` _array_element_4
                    (:`Is Valid`
                      (`/Game/GameModes/Battle/BP_BattlePC.BackToLobby` _array_element_4)))))
              (:`then_2`
                (bind _returnvalue (`GameplayStatics.GetCurrentLevelName` true))
                (`GameplayStatics.OpenLevel` (`KismetStringLibrary.Conv_StringToName` _returnvalue) true "listen")))
            (else
              (`self.SayToAll` (`KismetTextLibrary.Conv_TextToString` (`|FormatText` "{T} 후에 로비로 이동합니다." (`self.FormatMinSec` _result_2)))))))))))

(event `OnCharacterDeath`
  (params (PC :type "/Game/GameModes/Battle/BP_BattlePC Object Reference"))
  (`/Game/GameModes/Battle/BP_BattlePC.ShowDeathResult` PC (`KismetArrayLibrary.Array_Length` (`self.AlivePCs`)))
  (`KismetArrayLibrary.Array_RemoveItem` (`self.AlivePCs`) PC)
  (`KismetArrayLibrary.Array_Add` (`self.DeadPCs`) PC))

(event `AllDive`
  (for _array_element (`self.AlivePCs`)
    (`/Engine/EditorBlueprintResources/StandardMacros.IsValid` _array_element
      (:`Is Valid`
        (if (not (`/Game/GameModes/Battle/BP_BattlePC.Dived` _array_element))
          (`/Game/GameModes/Battle/BP_BattlePC.WantToDive` _array_element))))))

(fn `FormatMinSec`
  (params (Sec :type Integer))
  (returns (TimeText :type Text))
  (locals (Text :type String))
  (bind _returnvalue (/ Sec 60))
  (bind _returnvalue_2 (mod Sec 60))
  (if (not (== _returnvalue 0))
    (set `local.Text` (`KismetStringLibrary.Concat_StrStr` (`KismetStringLibrary.Conv_IntToString` _returnvalue) "분 ")))
  (if (not (== _returnvalue_2 0))
    (bind _output_get (set `local.Text` (`KismetStringLibrary.Concat_StrStr` (`local.Text`) (`KismetStringLibrary.Conv_IntToString` _returnvalue_2) "초"))))
  (return (`KismetTextLibrary.Conv_StringToText` _output_get)))

(fn `SayToAll`
  (params (Message :type String))
  (`|ExecutionSequence`
    (:`then_0`
      (for _array_element (`self.AlivePCs`)
        (`/Engine/EditorBlueprintResources/StandardMacros.IsValid` _array_element
          (:`Is Valid`
            (set `/Game/GameModes/Battle/BP_BattlePC.NotificationFromServer` Message _array_element)))))
    (:`then_1`
      (for _array_element_2 (`self.DeadPCs`)
        (`/Engine/EditorBlueprintResources/StandardMacros.IsValid` _array_element_2
          (:`Is Valid`
            (set `/Game/GameModes/Battle/BP_BattlePC.NotificationFromServer` Message _array_element_2)))))))

(fn `UserConstructionScript`)