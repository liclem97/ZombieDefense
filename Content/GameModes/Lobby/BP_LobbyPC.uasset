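; Player controller for the lobby, which presents the lobby menu and handles joining a server.
; On BeginPlay it plays music, then switches view to the camera tagged MainCamera and, if that succeeds, shows the lobby widget with UI-only input and a visible cursor.
; JoinServer opens the Loading level, passing the IP address as the NextMap option rather than connecting directly.
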(event `JoinServer`
  (params (IpAddress :type String))
  (`GameplayStatics.OpenLevel` "Loading" true (`KismetStringLibrary.Concat_StrStr` "NextMap=" IpAddress)))

(event `self.ReceiveBeginPlay`
  (`GameplayStatics.PlaySound2D` "/Game/BGM/bensound-epic_Cue.bensound-epic_Cue")
  (bind _outactors (`GameplayStatics.GetAllActorsWithTag` "MainCamera"))
  (if (> (`KismetArrayLibrary.Array_Length` _outactors) 0)
    (bind _ascamera_actor (cast `CameraActor` (`|GetArrayItem` _outactors)))
    (`self.SetViewTargetWithBlend` _ascamera_actor)
    (bind _returnvalue (`|CreateWidget` "/Game/GameModes/Lobby/WidgetBP_Lobby.WidgetBP_Lobby_C" self))
    (bind _output_get (set `self.WidgetBP_Lobby` _returnvalue))
    (`UserWidget.AddToViewport` _output_get 0)
    (`WidgetBlueprintLibrary.SetInputMode_UIOnlyEx` self _output_get)
    (set `self.bShowMouseCursor` true)))

(fn `OnRep_Name`)

(fn `UserConstructionScript`)