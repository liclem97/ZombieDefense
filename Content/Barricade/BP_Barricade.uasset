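; BP_Barricade is a damageable barricade that draws zombies to attack it until it is destroyed.
; Box overlap sets a BP_ZombieDefault's MainTarget to the barricade.
; Damage lowers HP; at zero, the last cast zombie is retargeted to Target and the actor is destroyed after a delay.
; A request event relays to a multicast, where WhichComputer limits the explosion emitter to the Other Client branch.
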(event `self.ReceiveBeginPlay`
  (`ActorComponent.Deactivate` (`self.Particle`)))

(event `self.Box.OnComponentBeginOverlap`
  (params (OverlappedComponent :type "PrimitiveComponent Object Reference") (OtherActor :type "Actor Object Reference") (OtherComp :type "PrimitiveComponent Object Reference") (OtherBodyIndex :type Integer) (bFromSweep :type Boolean) (SweepResult :type "HitResult Structure (by ref)"))
  (bind _asbp_zombie_default (cast `/Game/Enemy/Zombie/BP_ZombieDefault` OtherActor))
  (if (== OtherActor _asbp_zombie_default)
    (set `/Game/Enemy/Zombie/BP_ZombieDefault.MainTarget` self _asbp_zombie_default)))

(event `self.ReceiveAnyDamage`
  (params (Damage :type "Float (single-precision)") (DamageType :type "DamageType Object Reference") (InstigatedBy :type "Controller Object Reference") (DamageCauser :type "Actor Object Reference"))
  (`KismetSystemLibrary.PrintString` "Barricade Damaged")
  (bind _output_get (set `self.HP` (- (`self.HP`) Damage)))
  (if (<= _output_get 0.0)
    (set `/Game/Enemy/Zombie/BP_ZombieDefault.MainTarget` (`self.Target`) (stale `self.Box.OnComponentBeginOverlap` _asbp_zombie_default))
    (`self.ShowDestroyEffect_Req`)
    (`KismetSystemLibrary.Delay` 1.0)
    (`self.K2_DestroyActor`)))

(event `ShowDestroyEffect_Req`
  (`self.ShowDestroyEffect_Multicast`))

(event `ShowDestroyEffect_Multicast`
  (`self.WhichComputer`
    (:`OtherClient`
      (`GameplayStatics.SpawnEmitterAtLocation` "/Game/StarterContent/Particles/P_Explosion.P_Explosion" (`self.K2_GetActorLocation`) (struct) (5.0 5.0 5.0)))))

(fn `OnRep_Destroyed`)

(fn `UserConstructionScript`)