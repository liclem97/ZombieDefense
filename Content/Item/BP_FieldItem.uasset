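; BP_FieldItem is an item placed in the world that shows the mesh of its item class.
; On BeginPlay it uses its set ItemClassID or, if Random, the authority picks one from RandomItems, with the RepNotify triggering the mesh load.
; The load looks up ItemClassTable, async-loads the static mesh, rotates it by equip type (weapons pitched 90 degrees) and fits the Sphere radius to its bounds.
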(event `self.ReceiveBeginPlay`
  (bind _staticmeshcomponent (`self.StaticMeshComponent`))
  (bind _returnvalue (`KismetArrayLibrary.Array_Length` (`self.RandomItems`)))
  (if (`self.bRandom`)
    (`/Engine/EditorBlueprintResources/ActorMacros.Switch Has Authority`
      (:`Authority`
        (if (>= _returnvalue 1)
          (set `self.ItemClassID` (`|GetArrayItem` (`self.RandomItems`) (`KismetMathLibrary.RandomIntegerInRange` 0 (- _returnvalue 1)))))))
    (else
      (if (!= (`self.ItemClassID`) 0) :!label _label
        (bind _returnvalue_2 (`|GetDataTableRow` "/Game/Item/ItemClassTable.ItemClassTable" (`KismetStringLibrary.Conv_StringToName` (`KismetStringLibrary.Conv_IntToString` (`self.ItemClassID`))))
          (:`then`
            (bind (_itemclassid _itemname _itemequiptype _skeletalmesh _staticmesh) (break `/Game/Item/ItemClass` _returnvalue_2))
            (bind _object (`|LoadAsset` _staticmesh)
              (:`then`
                (switch `/Game/Item/EItemEquipType` _itemequiptype
                  (:`NewEnumerator0`
                    (`SceneComponent.K2_SetRelativeRotation` :`self` (`self.StaticMeshComponent`) :!label _label_2))
                  (:`NewEnumerator1`
                    (goto _label_2))
                  (:`NewEnumerator2`
                    (goto _label_2))
                  (:`NewEnumerator3`
                    (goto _label_2))
                  (:`NewEnumerator4`
                    (`SceneComponent.K2_SetRelativeRotation` (`self.StaticMeshComponent`) (struct :`Roll` 90.0) false false))))
              (:`Completed`
                (bind _asstatic_mesh (cast `StaticMesh` _object))
                (`StaticMeshComponent.SetStaticMesh` _staticmeshcomponent _asstatic_mesh)
                (`SphereComponent.SetSphereRadius` (`self.Sphere`) (`.SphereRadius` (`KismetSystemLibrary.GetComponentBounds` _staticmeshcomponent)) true)))))))))

(event `LoadItemMesh`
  (goto _label))

(fn `OnRep_ItemClassID`
  (`self.LoadItemMesh`))

(fn `UserConstructionScript`)