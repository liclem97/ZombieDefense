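; BP_Nexus is the objective zombies attack: a floating diamond with lights and an HP pool that it reports to BP_ZombieGM.
; Damage lowers HP and switches the diamond material and lights to green or red by threshold.
; Tick bobs the diamond with a sine and, once HP hits zero, triggers explosion, hiding, break and lose sounds.
; Box overlaps toggle AttackTarget on tagged zombies and bosses.
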(event `self.ReceiveTick`
  (params (DeltaSeconds :type "Float (single-precision)"))
  (`|ExecutionSequence`
    (:`then_0`
      (bind _output_get (set `self.RunningTime` (+ DeltaSeconds (`self.RunningTime`))))
      (bind _output_get_2 (set `self.Location` (`KismetMathLibrary.MakeVector` (.x (`SceneComponent.K2_GetComponentLocation` (`self.Diamond`))) (.y (`SceneComponent.K2_GetComponentLocation` (`self.Diamond`))) (+ (/ (`KismetMathLibrary.Sin` _output_get) 5.0) (.z (`SceneComponent.K2_GetComponentLocation` (`self.Diamond`)))))))
      (`SceneComponent.K2_SetWorldLocation` (`self.Diamond`) _output_get_2 false false))
    (:`then_1`
      (if (<= (`self.HP`) 0.0)
        (`/Engine/EditorBlueprintResources/StandardMacros.DoOnce` false
          (:`Completed`
            (`self.PlayDestroy`)))))))

(event `self.ReceiveBeginPlay`
  (`|ExecutionSequence`
    (:`then_0`
      (bind _asbp_zombie_gm (cast `/Game/GameModes/Zombie/BP_ZombieGM` (`GameplayStatics.GetGameMode`)))
      (set `self.GameMode` _asbp_zombie_gm))
    (:`then_1`
      (`/Game/GameModes/Zombie/BP_ZombieGM.UpdateNexusHP` (`self.GameMode`) (`self.HP`)))
    (:`then_2`
      (`ActorComponent.Deactivate` (`self.P_Explosion_Big_C`)))))

(event `ChangeColor_Green`
  (`LightComponent.SetLightColor` (`self.PointLight`) (`self.LightColor_Green`) true)
  (`LightComponent.SetLightColor` (`self.SpotLight`) (`self.LightColor_Green`) true)
  (`PrimitiveComponent.SetMaterial` (`self.Diamond`) 0 "/Game/Nexus/Texture/M_DemoWall_green.M_DemoWall_green"))

(event `self.ReceivePointDamage`
  (params (Damage :type "Float (single-precision)") (DamageType :type "DamageType Object Reference") (HitLocation :type "Vector Structure") (HitNormal :type "Vector Structure") (HitComponent :type "PrimitiveComponent Object Reference") (BoneName :type Name) (ShotFromDirection :type "Vector Structure") (InstigatedBy :type "Controller Object Reference") (DamageCauser :type "Actor Object Reference") (HitInfo :type "HitResult Structure (by ref)")))

(event `self.ReceiveAnyDamage`
  (params (Damage :type "Float (single-precision)") (DamageType :type "DamageType Object Reference") (InstigatedBy :type "Controller Object Reference") (DamageCauser :type "Actor Object Reference"))
  (bind _hp (`self.HP`))
  (bind _returnvalue (- (`self.Hp`) Damage))
  ;[1 1 1] PointDamage
  (if (<= _returnvalue 0.0)
    (set `self.HP` 0.0)
    (else
      (bind _output_get (set `self.HP` _returnvalue))))
  (`/Game/GameModes/Zombie/BP_ZombieGM.UpdateNexusHP` (`self.GameMode`) _output_get)
  (if (and (> _hp 200.0) (< _hp 400.0))
    (`self.ChangeColor_Green`)
    (elif (< (`self.HP`) 200.0)
      (`self.ChangeColor_Red`)
      (elif (<= (`self.HP`) 0.0)
        _))))

(event `ChangeColor_Red`
  (`LightComponent.SetLightColor` (`self.PointLight`) (`self.LightColor_Red`) true)
  (`LightComponent.SetLightColor` (`self.SpotLight`) (`self.LightColor_Red`) true)
  (`PrimitiveComponent.SetMaterial` (`self.Diamond`) 0 "/Game/Nexus/Texture/M_DemoWall_Red.M_DemoWall_Red"))

(event `PlayDestroy`
  (bind _p_explosion_big_c (`self.P_Explosion_Big_C`))
  (`ActorComponent.Activate` _p_explosion_big_c false)
  (`ActorComponent.SetActive` _p_explosion_big_c true false)
  (`SceneComponent.SetHiddenInGame` (`self.Diamond`) true false)
  (`GameplayStatics.PlaySoundAtLocation` "/Game/Sound/Nexus_Break.Nexus_Break" (`SceneComponent.K2_GetComponentLocation` (`self.Diamond`)) (struct) 1.0 1.0 0.45)
  (`KismetSystemLibrary.Delay` 1.0)
  (`GameplayStatics.PlaySound2D` "/Game/Sound/lose.lose"))

(event `self.Box.OnComponentBeginOverlap`
  (params (OverlappedComponent :type "PrimitiveComponent Object Reference") (OtherActor :type "Actor Object Reference") (OtherComp :type "PrimitiveComponent Object Reference") (OtherBodyIndex :type Integer) (bFromSweep :type Boolean) (SweepResult :type "HitResult Structure (by ref)"))
  (if (`self.ActorHasTag` OtherActor "Zombie")
    (`|ExecutionSequence`
      (:`then_0`
        (bind _asbp_zombie_default (cast `/Game/Enemy/Zombie/BP_ZombieDefault` OtherActor))
        (set `/Game/Enemy/Zombie/BP_ZombieDefault.AttackTarget` true _asbp_zombie_default))
      (:`then_1`
        (bind _asbp_boss (cast `/Game/Enemy/Boss/BP_Boss` OtherActor))
        (set `/Game/Enemy/Boss/BP_Boss.AttackTarget` true _asbp_boss)))))

(event `self.Box.OnComponentEndOverlap`
  (params (OverlappedComponent :type "PrimitiveComponent Object Reference") (OtherActor :type "Actor Object Reference") (OtherComp :type "PrimitiveComponent Object Reference") (OtherBodyIndex :type Integer))
  (if (`self.ActorHasTag` OtherActor "Zombie")
    (`|ExecutionSequence`
      (:`then_0`
        (bind _asbp_zombie_default (cast `/Game/Enemy/Zombie/BP_ZombieDefault` OtherActor))
        (set `/Game/Enemy/Zombie/BP_ZombieDefault.AttackTarget` false _asbp_zombie_default))
      (:`then_1`
        (bind _asbp_boss (cast `/Game/Enemy/Boss/BP_Boss` OtherActor))
        (set `/Game/Enemy/Boss/BP_Boss.AttackTarget` false _asbp_boss)))))

(fn `UserConstructionScript`)