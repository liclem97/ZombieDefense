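; BP_EnemySpawner is an enemy spawner actor that spawns a given enemy class in batches.
; SpawnerInit resets the count and stop flag, then SpawnEnemy spawns each batch with a fixed delay in its loop.
; It re-calls itself after SpawnDelay until the count reaches MaxSpawn.
; Repeat calls use the spawner's own transform and pass MaxSpawned, only ever set to zero here, as the limit.
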(event `SpawnerInit`
  (set `self.Spawned` 0)
  (set `self.MaxSpawned` 0)
  (set `self.IsStop` false))

(event `SpawnEnemy`
  (params (Enemy :type "Actor Class Reference") (SpawnTransform :type "Transform Structure") (`Num Of Enemies` :type Integer) (SpawnDelay :type "Float (double-precision)") (MaxSpawn :type Integer))
  (if (not (`self.IsStop`))
    (for _ (range `Num Of Enemies`)
      (`|SpawnActorFromClass` Enemy SpawnTransform "AdjustIfPossibleButAlwaysSpawn" "OverrideRootScale" null null)
      (set `self.Spawned` (+ (`self.Spawned`) 1))
      (`KismetSystemLibrary.Delay` 2.0))
    (if (>= (`self.Spawned`) MaxSpawn)
      (set `self.IsStop` true)
      (else
        (`KismetSystemLibrary.Delay` SpawnDelay)
        (`self.SpawnEnemy` (`self.Enemy`) (`self.GetTransform`) (`self.NumOfEnemies`) (`self.SpawnDelay`) (`self.MaxSpawned`))))))

(fn `UserConstructionScript`)