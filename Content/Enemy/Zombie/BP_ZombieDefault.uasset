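; Networked zombie enemy that chases the game mode's main target or its latest attacker, damaging players and the Nexus.
; A Tick state machine, enabled by OnRep_Target, runs follow, attack, stun and death, with two collision spheres live during attack animations.
; Point damage adds headshot bonuses, causes a one-time stun, and credits kills before ragdoll death.
; RepNotifies and multicasts sync speed, animations and effects; the wave-upgrade hook is disconnected.
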(event `self.ReceiveBeginPlay`
  (`|ExecutionSequence`
    (:`then_0`
      (`self.SetActorTickEnabled` false))
    (:`then_1`
      (bind _asbp_zombie_gm (cast `/Game/GameModes/Zombie/BP_ZombieGM` (`GameplayStatics.GetGameMode`)))
      (bind _output_get (set `self.GameMode` _asbp_zombie_gm))
      (bind _output_get_2 (set `self.MainTarget` (`/Game/GameModes/Zombie/BP_ZombieGM.MainTarget` _output_get)))
      (set `self.SubTarget` _output_get_2))
    (:`then_2`
      (bind _asbp_zombie_pc (cast `/Game/GameModes/Zombie/BP_ZombiePC` (`GameplayStatics.GetPlayerController` 0)))
      (set `self.PlayerController` _asbp_zombie_pc))
    (:`then_3`
      (`/Game/GameModes/Zombie/BP_ZombiePC.IncreaseZombie` (`self.PlayerController`)))
    (:`then_4`
      (`KismetSystemLibrary.K2_SetTimerDelegate` (delegate `ResetMainTarget`) 3.0 true))
    (:`then_5`
      (`self.Upgrade`))))

(event `Move`
  (bind _maintarget (`self.MainTarget`))
  (if (not (`self.IsAttacking`))
    (`/Engine/EditorBlueprintResources/StandardMacros.IsValid` _maintarget
      (:`Is Valid`
        (`|AIMoveTo` self (`self.K2_GetActorLocation` _maintarget) _maintarget 0.0)))))

(event `ResetMainTarget`
  (`/Engine/EditorBlueprintResources/StandardMacros.IsValid` (`self.MainTarget`)
    (:`Is Not Valid`
      (set `self.MainTarget` (`self.SubTarget`)))))

(event `PlayAttackAnim_Req`
  (`self.PlayAttackAnim_Multicast`))

(event `PlayAttackAnim_Multicast`
  (`self.PlayAnimMontage` "/Game/Enemy/Zombie/AnimMontage/zombie_attack_Montage.zombie_attack_Montage"))

(event `self.ReceiveTick`
  (params (DeltaSeconds :type "Float (single-precision)"))
  (`self.SaveDisAndDir`)
  (switch `/Game/Enemy/EnemyState` (`self.ZombieState`)
    (:`NewEnumerator0`
      (if (or (<= (`self.DistancePlayerChar`) (`self.AttackRange`)) (`self.AttackTarget`))
        (set `self.ZombieState` "NewEnumerator1")
        (`self.PlayAttackAnim_Req`)
        (set `self.IsAttacking` true)
        (elif (not (or (`self.IsAttacking`) (`self.IsStun`)))
          (`self.Move`))))
    (:`NewEnumerator1`
      (if (`self.IsAttacking`)
        _
        (elif (or (<= (`self.DistancePlayerChar`) (`self.AttackRange`)) (`self.AttackTarget`))
          (`self.PlayAttackAnim_Req`)
          (set `self.IsAttacking` true)
          (else
            (set `self.IsAttacking` false)
            (set `self.ZombieState` "NewEnumerator0")))))
    (:`NewEnumerator3`
      (set `self.IsAttacking` false)
      (set `self.IsStun` true)
      (`KismetSystemLibrary.Delay` 2.0)
      (set `self.IsStun` false)
      (set `self.ZombieState` "NewEnumerator0"))
    (:`NewEnumerator2`
      (`KismetSystemLibrary.Delay` 5.0)
      (`self.K2_DestroyActor`))))

(event `OnAnimStart_Attack`
  (if (not (`self.IsStun`))
    (set `self.IsAttacking` true)
    (`PrimitiveComponent.SetCollisionEnabled` (`self.Sphere`) "QueryAndPhysics")
    (`PrimitiveComponent.SetCollisionEnabled` (`self.Sphere1`) "QueryAndPhysics")
    (`self.PlayAttackSound`)))

(event `OnAnimEnd_Attack`
  (set `self.IsAttacking` false)
  (`PrimitiveComponent.SetCollisionEnabled` (`self.Sphere`) "NoCollision")
  (`PrimitiveComponent.SetCollisionEnabled` (`self.Sphere1`) "NoCollision")
  (set `self.ZombieState` "NewEnumerator0"))

(event `ApplyPointDamagePlayer_Req`
  (params (DamagedCharacter :type "/Game/Characters/BP_PlayerBase Object Reference") (BaseDamage :type "Float (double-precision)") (HitFromDirection :type "Vector Structure") (HitBoneName :type Name))
  ;[1 1 1] ApplyPointDamage
  (`GameplayStatics.ApplyPointDamage` DamagedCharacter BaseDamage HitFromDirection (`GameplayStatics.MakeHitResult` false false 0.0 0.0 (0.0 0.0 0.0) (0.0 0.0 0.0) (0.0 0.0 1.0) (0.0 0.0 1.0) null null null HitBoneName) (`self.GetController`) (cast `/Game/Enemy/Zombie/BP_ZombieDefault` (`GameplayStatics.GetPlayerCharacter` 0) :!pure true)))

(event `ApplyPointDamageNexus_Req`
  (params (DamagedActor :type "/Game/Nexus/BP_Nexus Object Reference") (BaseDamage :type "Float (double-precision)") (HitFromDirection :type "Vector Structure (by ref)") (HitBoneName :type Name))
  ;[1 1 1] ApplyPointDamage
  (`GameplayStatics.ApplyPointDamage` DamagedActor BaseDamage HitFromDirection (`GameplayStatics.MakeHitResult` false false 0.0 0.0 (0.0 0.0 0.0) (0.0 0.0 0.0) (0.0 0.0 1.0) (0.0 0.0 1.0) null null null HitBoneName) (`self.GetController`) (cast `/Game/Enemy/Zombie/BP_ZombieDefault` (`GameplayStatics.GetPlayerCharacter` 0) :!pure true)))

(event `ApplyAnyDamagePlayer_Req`
  (params (DamagedActor :type "/Game/Characters/BP_PlayerBase Object Reference") (BaseDamage :type "Float (double-precision)"))
  ;[1 1 1] ApplyAnyDamage
  (`GameplayStatics.ApplyDamage` DamagedActor BaseDamage (`self.GetController`) (cast `/Game/Enemy/Zombie/BP_ZombieDefault` (`GameplayStatics.GetPlayerCharacter` 0) :!pure true)))

(event `self.Sphere.OnComponentBeginOverlap`
  (params (OverlappedComponent :type "PrimitiveComponent Object Reference") (OtherActor :type "Actor Object Reference") (OtherComp :type "PrimitiveComponent Object Reference") (OtherBodyIndex :type Integer) (bFromSweep :type Boolean) (SweepResult :type "HitResult Structure (by ref)"))
  ;[1 1 1] Sphere Overlap
  (`|ExecutionSequence`
    (:`then_0`
      (bind _asbp_player_base (cast `/Game/Characters/BP_PlayerBase` OtherActor))
      (if (`self.ActorHasTag` _asbp_player_base "Player")
        (`self.ApplyAnyDamagePlayer_Req` _asbp_player_base (`self.Damage`))
        (bind _returnvalue (`self.K2_GetActorLocation` _asbp_player_base))
        (`GameplayStatics.SpawnEmitterAtLocation` "/Game/WeaponEffects/P_body_bullet_impact.P_body_bullet_impact" _returnvalue (struct) (2.0 2.0 2.0))
        (`self.ShowAttackEffect_Req` true _returnvalue)))
    (:`then_1`
      (bind _asbp_nexus (cast `/Game/Nexus/BP_Nexus` OtherActor))
      (`self.ApplyAnyDamageNexus_Req` _asbp_nexus (`self.Damage`))
      (bind _returnvalue_2 (`self.K2_GetActorLocation` _asbp_nexus))
      (`GameplayStatics.SpawnEmitterAtLocation` "/Game/WeaponEffects/P_body_bullet_impact.P_body_bullet_impact" _returnvalue_2 (struct) (2.0 2.0 2.0))
      (`self.ShowAttackEffect_Req` false _returnvalue_2))))

(event `ApplyAnyDamageNexus_Req`
  (params (DamagedActor :type "/Game/Nexus/BP_Nexus Object Reference") (BaseDamage :type "Float (double-precision)"))
  ;[1 1 1] ApplyAnyDamage
  (`GameplayStatics.ApplyDamage` DamagedActor BaseDamage (`self.GetController`) (cast `/Game/Enemy/Zombie/BP_ZombieDefault` (`GameplayStatics.GetPlayerCharacter` 0) :!pure true)))

(event `self.Sphere1.OnComponentBeginOverlap`
  (params (OverlappedComponent :type "PrimitiveComponent Object Reference") (OtherActor :type "Actor Object Reference") (OtherComp :type "PrimitiveComponent Object Reference") (OtherBodyIndex :type Integer) (bFromSweep :type Boolean) (SweepResult :type "HitResult Structure (by ref)"))
  ;[1 1 1] Sphere Overlap
  (`|ExecutionSequence`
    (:`then_0`
      (bind _asbp_player_base (cast `/Game/Characters/BP_PlayerBase` OtherActor))
      (if (`self.ActorHasTag` "Player")
        (`self.ApplyAnyDamagePlayer_Req` _asbp_player_base (`self.Damage`))
        (bind _returnvalue (`self.K2_GetActorLocation` _asbp_player_base))
        (`GameplayStatics.SpawnEmitterAtLocation` "/Game/WeaponEffects/P_body_bullet_impact.P_body_bullet_impact" _returnvalue (struct) (2.0 2.0 2.0))
        (`self.ShowAttackEffect_Req` true _returnvalue)))
    (:`then_1`
      (bind _asbp_nexus (cast `/Game/Nexus/BP_Nexus` OtherActor))
      (`self.ApplyAnyDamageNexus_Req` _asbp_nexus (`self.Damage`))
      (bind _returnvalue_2 (`self.K2_GetActorLocation` _asbp_nexus))
      (`GameplayStatics.SpawnEmitterAtLocation` "/Game/WeaponEffects/P_body_bullet_impact.P_body_bullet_impact" _returnvalue_2 (struct) (2.0 2.0 2.0))
      (`self.ShowAttackEffect_Req` false _returnvalue_2))))

(event `self.ReceivePointDamage`
  (params (Damage :type "Float (single-precision)") (DamageType :type "DamageType Object Reference") (HitLocation :type "Vector Structure") (HitNormal :type "Vector Structure") (HitComponent :type "PrimitiveComponent Object Reference") (BoneName :type Name) (ShotFromDirection :type "Vector Structure") (InstigatedBy :type "Controller Object Reference") (DamageCauser :type "Actor Object Reference") (HitInfo :type "HitResult Structure (by ref)"))
  ;[1 1 1] PointDamage
  (bind _output_get (set `self.HP` (- (`self.HP`) Damage)))
  (if (== BoneName "Head")
    (set `self.HP` (- (`self.HP`) (* Damage 2.0))))
  (if (<= _output_get 0.0)
    (`self.WhichComputer`
      (:`Server`
        _)
      (:`MyClient`
        _)
      (:`OtherClient`
        _))
    (`self.DeathAnimation_Multicast`)
    (if (not (`self.Death`))
      (bind _asbp_player_base (cast `/Game/Characters/BP_PlayerBase` DamageCauser))
      (`/Game/Characters/BP_PlayerBase.KillZombie` _asbp_player_base)
      (set `self.ZombieState` "NewEnumerator2")
      (set `self.Death` true))
    (else
      (if (<= (`self.HP`) 80.0)
        _
        (else
          _))
      (set `self.MainTarget` DamageCauser)
      (`/Engine/EditorBlueprintResources/StandardMacros.DoOnce` false
        (:`Completed`
          (set `self.ZombieState` "NewEnumerator3"))))))

(event `UpgradeZombie`
  (bind _mesh (`self.Mesh`))
  (bind _charactermovement (`self.CharacterMovement`))
  ;[1 1 1] PointDamage
  (`PrimitiveComponent.SetMaterial` _mesh 0 "/Game/Enemy/Zombie/Ch10_body_Inst.Ch10_body_Inst")
  (`PrimitiveComponent.SetMaterial` _mesh 1 "/Game/Enemy/Zombie/Ch10_body1_Inst.Ch10_body1_Inst")
  (set `CharacterMovementComponent.MaxWalkSpeed` (+ (`CharacterMovementComponent.MaxWalkSpeed` _charactermovement) 100.0) _charactermovement)
  (set `self.Damage` (* (`self.Damage`) 2.0)))

(event `PlayAttackSound`
  (`GameplayStatics.PlaySoundAtLocation` "/Game/Sound/zombieeating-85423.zombieeating-85423" (`self.K2_GetActorLocation`)))

(event `Upgrade`)

(event `ShowAttackEffect_Req`
  (params (IsHuman :type Boolean) (SpawnLocation :type "Vector Structure"))
  (`self.ShowAttackEffect_Multicast` IsHuman SpawnLocation))

(event `DeathAnimation_Multicast`
  (`PrimitiveComponent.SetSimulatePhysics` (`self.Mesh`) true)
  (`|ExecutionSequence`
    (:`then_0`
      (`SkeletalMeshComponent.SetAllBodiesBelowPhysicsBlendWeight` (`self.Mesh`) "Hips" 1.0 false true)
      (`PrimitiveComponent.SetCollisionEnabled` (`self.CapsuleComponent`) "NoCollision")
      (`CharacterMovementComponent.SetMovementMode` (`self.CharacterMovement`) "MOVE_None" 0))))

(event `ShowAttackEffect_Multicast`
  (params (IsHuman :type Boolean) (SpawnLocation :type "Vector Structure"))
  (`self.WhichComputer`
    (:`OtherClient`
      (if IsHuman
        (`GameplayStatics.SpawnEmitterAtLocation` "/Game/WeaponEffects/P_body_bullet_impact.P_body_bullet_impact" SpawnLocation (struct) (2.0 2.0 2.0))
        (else
          (`GameplayStatics.SpawnEmitterAtLocation` "/Game/WeaponEffects/P_AssaultRifle_IH.P_AssaultRifle_IH" SpawnLocation))))))

(event `Attack`
  ;[1 1 1] Attack
)

(fn `OnRep_Death`
  (`|ExecutionSequence`
    (:`then_0`
      (`GameplayStatics.PlaySoundAtLocation` "/Game/Sounds_StrategyGame/Characters/Voiceovers/VO_Jose_death10.VO_Jose_death10" (`self.K2_GetActorLocation`))
      (`PrimitiveComponent.SetCollisionEnabled` (`self.CapsuleComponent`) "NoCollision")
      (`CharacterMovementComponent.SetMovementMode` (`self.CharacterMovement`) "MOVE_None" 0))
    (:`then_1`
      (`/Game/GameModes/Zombie/BP_ZombiePC.DecreaseZombie` (`self.PlayerController`)))))

(fn `OnRep_IsAttacking`
  (if (`self.IsAttacking`)
    (set `CharacterMovementComponent.MaxWalkSpeed` 0.0 (`self.CharacterMovement`))
    (else
      (set `CharacterMovementComponent.MaxWalkSpeed` 150.0 (`self.CharacterMovement`)))))

(fn `OnRep_IsStun`
  (if (`self.IsStun`)
    (`/Engine/EditorBlueprintResources/StandardMacros.DoOnce` false
      (:`Completed`
        (set `CharacterMovementComponent.MaxWalkSpeed` 0.0 (`self.CharacterMovement`))
        (`self.PlayAnimMontage` "/Game/Enemy/Zombie/AnimMontage/zombie_reaction_hit_Montage2.zombie_reaction_hit_Montage2" 1.3)))
    (else
      (`self.StopAnimMontage` "/Game/Enemy/Zombie/AnimMontage/zombie_reaction_hit_Montage2.zombie_reaction_hit_Montage2")
      (set `CharacterMovementComponent.MaxWalkSpeed` 150.0 (`self.CharacterMovement`)))))

(fn `OnRep_Target`
  (`self.SetActorTickEnabled` true))

(fn `OnRep_TargetNum`)

(fn `SaveDisAndDir`
  (bind _maintarget (`self.MainTarget`))
  (bind _returnvalue (- (`self.K2_GetActorLocation` _maintarget) (`self.K2_GetActorLocation`)))
  (`/Engine/EditorBlueprintResources/StandardMacros.IsValid` _maintarget
    (:`Is Valid`
      _)
    (:`Is Not Valid`
      (bind _asbp_zombie_gm (cast `/Game/GameModes/Zombie/BP_ZombieGM` (`GameplayStatics.GetGameMode`)))
      (set `self.MainTarget` (`/Game/GameModes/Zombie/BP_ZombieGM.MainTarget` _asbp_zombie_gm))))
  (set `self.DistancePlayerChar` (`KismetMathLibrary.VSize` _returnvalue))
  (set `self.DirToPlayerChar` (`KismetMathLibrary.Normal` _returnvalue)))

(fn `UserConstructionScript`)