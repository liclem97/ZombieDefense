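; Networked zombie enemy character that melees players and barricades, takes bonus headshot damage, can be stunned, and ragdolls on death.
; Attack montage events trigger a line trace that applies point damage, with request events and multicasts for montages and effects.
; RepNotifies on attack, stun and death flags drive walk speed, reactions and collision.
; The distance-based follow/attack/stun/death state machine is disconnected, as Tick is empty.
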(event `self.ReceiveBeginPlay`)

(event `MoveToVector`
  (`|AIMoveTo` self (`self.TargetVector`) (`self.GetOwner`)))

(event `Move`
  (bind _target (`self.Target`))
  (if (not (`self.IsAttacking`))
    (`|AIMoveTo` self (`self.K2_GetActorLocation` _target) _target 0.0)))

(event `PlayAttackAnim_Req`
  (`self.PlayAttackAnim_Multicast`))

(event `PlayAttackAnim_Multicast`
  (`self.PlayAnimMontage` "/Game/Enemy/Zombie/AnimMontage/zombie_attack_Montage.zombie_attack_Montage" 1.3))

(event `self.ReceiveTick`
  (params (DeltaSeconds :type "Float (single-precision)")))

(event `OnAnimStart_Attack`
  (if (not (`self.IsStun`))
    (set `self.IsAttacking` true)
    (`self.Attack`)))

(event `DelaySec`
  (`KismetSystemLibrary.Delay` 10.0)
  (`KismetSystemLibrary.PrintString` "Hello"))

(event `OnAnimEnd_Attack`
  (set `self.IsAttacking` false)
  (set `self.ZombieState` "NewEnumerator0"))

(event `ApplyPointDamagePlayer_Req`
  (params (DamagedCharacter :type "/Game/Characters/BP_PlayerBase Object Reference") (BaseDamage :type "Float (double-precision)") (HitFromDirection :type "Vector Structure") (HitBoneName :type Name))
  (`GameplayStatics.ApplyPointDamage` DamagedCharacter BaseDamage HitFromDirection (`GameplayStatics.MakeHitResult` false false 0.0 0.0 (0.0 0.0 0.0) (0.0 0.0 0.0) (0.0 0.0 1.0) (0.0 0.0 1.0) null null null HitBoneName) (`self.GetController`) (cast `/Game/Enemy/Zombie/BP_ZombieDefault` (`GameplayStatics.GetPlayerCharacter` 0) :!pure true)))

(event `ApplyPointDamageBarricade_Req`
  (params (DamagedCharacter :type "/Game/Barricade/BP_Barricade Object Reference") (BaseDamage :type "Float (double-precision)") (HitFromDirection :type "Vector Structure") (HitBoneName :type Name))
  (`GameplayStatics.ApplyPointDamage` DamagedCharacter BaseDamage HitFromDirection (`GameplayStatics.MakeHitResult` false false 0.0 0.0 (0.0 0.0 0.0) (0.0 0.0 0.0) (0.0 0.0 1.0) (0.0 0.0 1.0) null null null HitBoneName) (`self.GetController`) (cast `/Game/Barricade/BP_Barricade` (`self.GetOwner`) :!pure true)))

(event `self.ReceivePointDamage`
  (params (Damage :type "Float (single-precision)") (DamageType :type "DamageType Object Reference") (HitLocation :type "Vector Structure") (HitNormal :type "Vector Structure") (HitComponent :type "PrimitiveComponent Object Reference") (BoneName :type Name) (ShotFromDirection :type "Vector Structure") (InstigatedBy :type "Controller Object Reference") (DamageCauser :type "Actor Object Reference") (HitInfo :type "HitResult Structure (by ref)"))
  (bind _output_get (set `self.HP` (- (`self.HP`) Damage)))
  (if (== BoneName "Head")
    (set `self.HP` (- (`self.HP`) (* Damage 2.0))))
  (if (<= _output_get 0.0)
    (`self.WhichComputer`
      (:`Server`
        _)
      (:`MyClient`
        _)
      (:`OtherClient`
        _))
    (`GameplayStatics.PlaySoundAtLocation` "/Game/Sounds_StrategyGame/Characters/Voiceovers/VO_Jose_death10.VO_Jose_death10" (`self.K2_GetActorLocation`) (struct) 1.0 1.0 0.0 null null null null)
    (`self.DeathAnimation_Multicast`)
    (set `self.Death` true)
    (set `self.ZombieState` "NewEnumerator2")
    (elif (== (`self.HP`) 50.0)
      (set `self.Target` DamageCauser)
      (set `self.ZombieState` "NewEnumerator3"))))

(event `ShowAttackEffect_Req`
  (params (IsHuman :type Boolean) (SpawnLocation :type "Vector Structure"))
  (`self.ShowAttackEffect_Multicast` IsHuman SpawnLocation))

(event `DeathAnimation_Multicast`
  (`PrimitiveComponent.SetSimulatePhysics` (`self.Mesh`) true)
  (`|ExecutionSequence`
    (:`then_0`
      (`SkeletalMeshComponent.SetAllBodiesBelowPhysicsBlendWeight` (`self.Mesh`) "Hips" 1.0 false true)
      (`PrimitiveComponent.SetCollisionEnabled` (`self.CapsuleComponent`) "NoCollision")
      (`CharacterMovementComponent.SetMovementMode` (`self.CharacterMovement`) "MOVE_None" 0))))

(event `ShowAttackEffect_Multicast`
  (params (IsHuman :type Boolean) (SpawnLocation :type "Vector Structure"))
  (`self.WhichComputer`
    (:`OtherClient`
      (if IsHuman
        (`GameplayStatics.SpawnEmitterAtLocation` "/Game/WeaponEffects/P_body_bullet_impact.P_body_bullet_impact" SpawnLocation (struct) (2.0 2.0 2.0))
        (else
          (`GameplayStatics.SpawnEmitterAtLocation` "/Game/WeaponEffects/P_AssaultRifle_IH.P_AssaultRifle_IH" SpawnLocation))))))

(event `Attack`
  (bind _returnvalue (`SceneComponent.K2_GetComponentLocation` (`self.LineTraceDummy`)))
  (bind _returnvalue_2 (`KismetMathLibrary.GetForwardVector` (`self.GetControlRotation`)))
  ;[1 1 1] Attack
  (bind (_outhit _returnvalue_3) (`KismetSystemLibrary.LineTraceSingleForObjects` _returnvalue (+ _returnvalue (* _returnvalue_2 (`self.AttackRange`))) (`|MakeArray` "ObjectTypeQuery1" "ObjectTypeQuery2" "ObjectTypeQuery4" "ObjectTypeQuery5" "ObjectTypeQuery6" :!type "EObjectTypeQuery Enum") true (`|MakeArray` self :!type "Actor Object Reference") "Persistent"))
  (if _returnvalue_3
    (bind (_bblockinghit _binitialoverlap _time _distance _location _impactpoint _normal _impactnormal _physmat _hitactor _hitcomponent _hitbonename) (`GameplayStatics.BreakHitResult` _outhit))
    (if (`KismetStringLibrary.EqualEqual_StrStr` (`KismetSystemLibrary.GetDisplayName` _hitactor) "BP_Barricade")
      (bind _asbp_barricade (cast `/Game/Barricade/BP_Barricade` _hitactor))
      (bind _returnvalue_4 (+ _impactpoint (* _impactnormal 20.0)))
      (`self.ApplyPointDamageBarricade_Req` _asbp_barricade 50.0 _returnvalue_4)
      (if (== (`/Game/Barricade/BP_Barricade.HP` _asbp_barricade) 0.0)
        (set `self.IsAttacking` false)
        (set `self.ZombieState` "NewEnumerator0"))
      (else
        (bind _asbp_player_base (cast `/Game/Characters/BP_PlayerBase` _hitactor))
        (if (`ActorComponent.ComponentHasTag` _hitcomponent "Body")
          (`self.ApplyPointDamagePlayer_Req` _asbp_player_base 1.0 _returnvalue_2 _hitbonename)
          (`GameplayStatics.SpawnEmitterAtLocation` "/Game/WeaponEffects/P_body_bullet_impact.P_body_bullet_impact" _returnvalue_4 (struct) (2.0 2.0 2.0))
          (`self.ShowAttackEffect_Req` true _returnvalue_4))))))

(fn `OnRep_Death`
  (`GameplayStatics.PlaySoundAtLocation` "/Game/Sounds_StrategyGame/Characters/Voiceovers/VO_Jose_death10.VO_Jose_death10" (`self.K2_GetActorLocation`) (struct) 1.0 1.0 0.0 null null null null)
  (`PrimitiveComponent.SetCollisionEnabled` (`self.CapsuleComponent`) "NoCollision")
  (`CharacterMovementComponent.SetMovementMode` (`self.CharacterMovement`) "MOVE_None" 0))

(fn `OnRep_IsAttacking`
  (if (`self.IsAttacking`)
    (set `CharacterMovementComponent.MaxWalkSpeed` 0.0 (`self.CharacterMovement`))
    (else
      (set `CharacterMovementComponent.MaxWalkSpeed` 150.0 (`self.CharacterMovement`)))))

(fn `OnRep_IsStun`
  (if (`self.IsStun`)
    (`/Engine/EditorBlueprintResources/StandardMacros.DoOnce` false
      (:`Completed`
        (set `CharacterMovementComponent.MaxWalkSpeed` 0.0 (`self.CharacterMovement`))
        (`self.PlayAnimMontage` "/Game/Enemy/Zombie/AnimMontage/zombie_reaction_hit_Montage2.zombie_reaction_hit_Montage2" 1.3)))
    (else
      (`self.StopAnimMontage` "/Game/Enemy/Zombie/AnimMontage/zombie_reaction_hit_Montage2.zombie_reaction_hit_Montage2")
      (set `CharacterMovementComponent.MaxWalkSpeed` 150.0 (`self.CharacterMovement`)))))

(fn `OnRep_TargetNum`)

(fn `SaveDisAndDir`
  (bind _target (`self.Target`))
  (bind _returnvalue (- (`self.TargetVector`) (`self.K2_GetActorLocation`)))
  (bind _returnvalue_2 (- (`self.K2_GetActorLocation` _target) (`self.K2_GetActorLocation`)))
  (`/Engine/EditorBlueprintResources/StandardMacros.IsValid` _target
    (:`Is Valid`
      (set `self.DistancePlayerChar` (`KismetMathLibrary.VSize` _returnvalue_2))
      (set `self.DirToPlayerChar` (`KismetMathLibrary.Normal` _returnvalue_2)))
    (:`Is Not Valid`
      (set `self.DistancePlayerChar` (`KismetMathLibrary.VSize` _returnvalue))
      (set `self.DirToPlayerChar` (`KismetMathLibrary.Normal` _returnvalue)))))

(fn `UserConstructionScript`)