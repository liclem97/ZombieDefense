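; BP_Boss is the replicated boss enemy of a zombie game, chasing and attacking players and the Nexus.
; A Tick state machine switches between follow, attack and death, choosing punch or skill montages on timer-driven cooldowns.
; Animation events toggle sphere and capsule overlaps that deal damage, while multicasts and RepNotifies sync animations, effects and state.
; Point damage adds headshot bonus, retargets the attacker and updates boss HP; death changes GameMode's playing state.
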(event `self.ReceiveBeginPlay`
  ;[1 1 1] BeginPlay & ResetMainTarget
  (`|ExecutionSequence`
    (:`then_0`
      (`self.SetActorTickEnabled` false :!label _label))
    (:`then_1`
      (goto _label))
    (:`then_2`
      (bind _asbp_zombie_gm (cast `/Game/GameModes/Zombie/BP_ZombieGM` (`GameplayStatics.GetGameMode`)))
      (bind _output_get (set `self.GameMode` _asbp_zombie_gm))
      (bind _output_get_2 (set `self.MainTarget` (`/Game/GameModes/Zombie/BP_ZombieGM.MainTarget` _output_get)))
      (set `self.SubTarget` _output_get_2))
    (:`then_3`
      (bind _asbp_zombie_pc (cast `/Game/GameModes/Zombie/BP_ZombiePC` (`GameplayStatics.GetPlayerController` 0)))
      (bind _output_get_3 (set `self.PlayerController` _asbp_zombie_pc))
      (`/Game/GameModes/Zombie/BP_ZombieGM.UpdateBossHP` (`self.GameMode`) (`self.Hp`))
      (`/Game/GameModes/Zombie/BP_ZombiePC.ShowBossUI` _output_get_3))
    (:`then_4`
      (`/Game/GameModes/Zombie/BP_ZombiePC.IncreaseZombie` (`self.PlayerController`)))
    (:`then_5`
      (`KismetSystemLibrary.K2_SetTimerDelegate` (delegate `ResetMainTarget`) 5.0 true))
    (:`then_6`
      (`KismetSystemLibrary.K2_SetTimerDelegate` (delegate `SkillCoolTime`) 1.0 true))
    (:`then_7`
      (`KismetSystemLibrary.K2_SetTimerDelegate` (delegate `AttackDelay`) 1.0 true))))

(event `Move`
  (bind _maintarget (`self.MainTarget`))
  ;[1 1 1] Move
  (if (not (`self.IsAttacking`))
    (`/Engine/EditorBlueprintResources/StandardMacros.IsValid` _maintarget
      (:`Is Valid`
        (`|AIMoveTo` self (`self.K2_GetActorLocation` _maintarget) _maintarget 0.0)))))

(event `self.ReceiveTick`
  (params (DeltaSeconds :type "Float (single-precision)"))
  ;[1 1 1] Tick
  (`/Engine/EditorBlueprintResources/StandardMacros.IsValid` (`self.MainTarget`)
    (:`Is Valid`
      (`self.SaveDisAndDir`)
      (switch `/Game/Enemy/EnemyState` (`self.EnemyState`)
        (:`NewEnumerator0`
          (if (or (<= (`self.DistancePlayerChar`) (`self.AttackRange`)) (`self.AttackTarget`))
            (set `self.EnemyState` "NewEnumerator1")
            (if (== (`self.SkillTime`) 0.0)
              (`self.PlaySkillAnim_Req`)
              (set `self.IsAttacking` true)
              (set `self.SkillTime` 15.0)
              (elif (== (`self.AttackTime`) 0.0)
                (`self.PlayAttackAnim_Req`)
                (set `self.IsAttacking` true)))
            (elif (not (`self.IsAttacking`))
              (set `CharacterMovementComponent.MaxWalkSpeed` (`self.MoveSpeed`) (`self.CharacterMovement`))
              (`self.Move`))))
        (:`NewEnumerator1`
          (if (`self.IsAttacking`)
            _
            (elif (or (<= (`self.DistancePlayerChar`) (`self.AttackRange`)) (`self.AttackTarget`))
              (if (== (`self.SkillTime`) 0.0)
                (`self.PlaySkillAnim_Req`)
                (set `self.IsAttacking` true)
                (set `self.SkillTime` 15.0)
                (elif (== (`self.AttackTime`) 0.0)
                  (`self.PlayAttackAnim_Req`)
                  (set `self.IsAttacking` true)))
              (else
                (set `self.IsAttacking` false)
                (set `self.EnemyState` "NewEnumerator0")))))
        (:`NewEnumerator2`
          (`KismetSystemLibrary.Delay` 7.0)
          (`self.K2_DestroyActor`))))))

(event `self.ReceivePointDamage`
  (params (Damage :type "Float (single-precision)") (DamageType :type "DamageType Object Reference") (HitLocation :type "Vector Structure") (HitNormal :type "Vector Structure") (HitComponent :type "PrimitiveComponent Object Reference") (BoneName :type Name) (ShotFromDirection :type "Vector Structure") (InstigatedBy :type "Controller Object Reference") (DamageCauser :type "Actor Object Reference") (HitInfo :type "HitResult Structure (by ref)"))
  ;[1 1 1] PointDamage
  (bind _output_get (set `self.HP` (- (`self.Hp`) Damage)))
  (if (== BoneName "Head")
    (set `self.HP` (- (`self.HP`) (* Damage 2.0))))
  (`/Game/GameModes/Zombie/BP_ZombieGM.UpdateBossHP` (`self.GameMode`) _output_get)
  (if (<= _output_get 0.0)
    (`self.WhichComputer`
      (:`Server`
        _)
      (:`MyClient`
        _)
      (:`OtherClient`
        _))
    (`self.DeathAnimation_Multicast`)
    (if (not (`self.Death`))
      (bind _asbp_player_base (cast `/Game/Characters/BP_PlayerBase` DamageCauser))
      (`/Game/Characters/BP_PlayerBase.KillZombie` _asbp_player_base)
      (set `self.EnemyState` "NewEnumerator2")
      (set `self.Death` true))
    (else
      (if (<= (`self.HP`) 80.0)
        _
        (else
          _))
      (set `self.MainTarget` DamageCauser))))

(event `ResetMainTarget`
  ;[1 1 1] BeginPlay & ResetMainTarget
  (`/Engine/EditorBlueprintResources/StandardMacros.IsValid` (`self.MainTarget`)
    (:`Is Not Valid`
      (set `self.MainTarget` (`self.SubTarget`)))))

(event `SkillCoolTime`
  ;[1 1 1] BeginPlay & ResetMainTarget
  (if (> (`self.SkillTime`) 0.0)
    (set `self.SkillTime` (- (`self.SkillTime`) 1.0))
    (else
      (set `self.SkillTime` 0.0))))

(event `AttackDelay`
  ;[1 1 1] BeginPlay & ResetMainTarget
  (if (> (`self.AttackTime`) 0.0)
    (set `self.AttackTime` (- (`self.AttackTime`) 1.0))
    (else
      (set `self.AttackTime` 0.0))))

(event `ShowAttackEffect_Req`
  (params (IsHuman :type Boolean) (SpawnLocation :type "Vector Structure"))
  ;[1 1 1] ShowAttackEffect
  (`self.ShowAttackEffect_Multicast` IsHuman SpawnLocation))

(event `DeathAnimation_Multicast`
  ;[1 1 1] DeathAnimation_Multicast
  (`/Engine/EditorBlueprintResources/StandardMacros.DoOnce` false
    (:`Completed`
      (`self.PlayAnimMontage` "/Game/Enemy/Boss/Boss1/AnimMontage/mutant_dying_Montage.mutant_dying_Montage"))))

(event `UpdateHP`
  (bind _gamemode (`self.GameMode`))
  (`/Engine/EditorBlueprintResources/StandardMacros.IsValid` _gamemode
    (:`Is Valid`
      (set `/Game/GameModes/Zombie/BP_ZombieGM.BossHP` (`self.Hp`) _gamemode)
      (set `/Game/GameModes/Zombie/BP_ZombieGM.BossMaxHP` (`self.MaxHP`) _gamemode))))

(event `OnAnimStart_Attack`
  ;[1 1 1] OnAnim
  (set `self.IsAttacking` false)
  (`PrimitiveComponent.SetCollisionEnabled` (`self.Sphere`) "QueryAndPhysics")
  (`self.PlaySoundPunch`))

(event `ApplyPointDamagePlayer_Req`
  (params (DamagedCharacter :type "/Game/Characters/BP_PlayerBase Object Reference") (BaseDamage :type "Float (double-precision)") (HitFromDirection :type "Vector Structure") (HitBoneName :type Name))
  ;[1 1 1] ApplyPointDamagePlayer_Req
  (`GameplayStatics.ApplyPointDamage` DamagedCharacter BaseDamage HitFromDirection (`GameplayStatics.MakeHitResult` false false 0.0 0.0 (0.0 0.0 0.0) (0.0 0.0 0.0) (0.0 0.0 1.0) (0.0 0.0 1.0) null null null HitBoneName) (`self.GetController`) (cast `/Game/Enemy/Boss/BP_Boss` (`GameplayStatics.GetPlayerCharacter` 0) :!pure true)))

(event `ApplyAnyDamagePlayer_Req`
  (params (DamagedActor :type "/Game/Characters/BP_PlayerBase Object Reference") (BaseDamage :type "Float (double-precision)"))
  ;[1 1 1] ApplyAnyDamage
  (`GameplayStatics.ApplyDamage` DamagedActor BaseDamage (`self.GetController`) (cast `/Game/Enemy/Boss/BP_Boss` (`GameplayStatics.GetPlayerCharacter` 0) :!pure true)))

(event `ApplyPointDamageNexus_Req`
  (params (DamagedActor :type "/Game/Nexus/BP_Nexus Object Reference") (BaseDamage :type "Float (double-precision)") (HitFromDirection :type "Vector Structure (by ref)") (HitBoneName :type Name))
  ;[1 1 1] ApplyPointDamagePlayer_Req
  (`GameplayStatics.ApplyPointDamage` DamagedActor BaseDamage HitFromDirection (`GameplayStatics.MakeHitResult` false false 0.0 0.0 (0.0 0.0 0.0) (0.0 0.0 0.0) (0.0 0.0 1.0) (0.0 0.0 1.0) null null null HitBoneName) (`self.GetController`) (cast `/Game/Enemy/Boss/BP_Boss` (`GameplayStatics.GetPlayerCharacter` 0) :!pure true)))

(event `ShowAttackEffect_Multicast`
  (params (IsHuman :type Boolean) (SpawnLocation :type "Vector Structure"))
  ;[1 1 1] ShowAttackEffect
  (`self.WhichComputer`
    (:`OtherClient`
      (if IsHuman
        (`GameplayStatics.SpawnEmitterAtLocation` "/Game/WeaponEffects/P_body_bullet_impact.P_body_bullet_impact" SpawnLocation (struct) (2.0 2.0 2.0))
        (else
          (`GameplayStatics.SpawnEmitterAtLocation` "/Game/WeaponEffects/P_AssaultRifle_IH.P_AssaultRifle_IH" SpawnLocation))))))

(event `OnAnimEnd_Attack`
  ;[1 1 1] OnAnim
  (set `self.IsAttacking` false)
  (`PrimitiveComponent.SetCollisionEnabled` (`self.Sphere`) "NoCollision")
  (set `self.EnemyState` "NewEnumerator0"))

(event `PlaySoundSword`
  (`GameplayStatics.PlaySoundAtLocation` "/Game/Sound/FightSword01_ImpactPound_Stereo.FightSword01_ImpactPound_Stereo" (`self.K2_GetActorLocation`)))

(event `ApplyAnyDamageNexus_Req`
  (params (DamagedActor :type "/Game/Nexus/BP_Nexus Object Reference") (BaseDamage :type "Float (double-precision)"))
  ;[1 1 1] ApplyAnyDamage
  (`GameplayStatics.ApplyDamage` DamagedActor BaseDamage (`self.GetController`) (cast `/Game/Enemy/Boss/BP_Boss` (`GameplayStatics.GetPlayerCharacter` 0) :!pure true)))

(event `OnAnimStart_Skill`
  ;[1 1 1] OnAnim
  (set `self.IsSkill` true)
  (set `self.IsAttacking` true)
  (`PrimitiveComponent.SetCollisionEnabled` (`self.Capsule1`) "QueryAndPhysics")
  (`self.PlaySoundSword`)
  (set `self.SkillTime` 20.0))

(event `PlaySoundPunch`
  (`GameplayStatics.PlaySoundAtLocation` "/Game/Sound/punch-2-123106.punch-2-123106" (`self.K2_GetActorLocation`)))

(event `OnAnimEnd_Skill`
  ;[1 1 1] OnAnim
  (set `self.IsSkill` false)
  (set `self.IsAttacking` false)
  (`PrimitiveComponent.SetCollisionEnabled` (`self.Capsule1`) "NoCollision")
  (set `self.EnemyState` "NewEnumerator0"))

(event `PlayAttackAnim_Req`
  ;[1 1 1] PlayAttackAnim
  (`self.PlayAttackAnim_Multicast`))

(event `PlayAttackAnim_Multicast`
  ;[1 1 1] PlayAttackAnim
  (`self.PlayAnimMontage` "/Game/Enemy/Boss/Boss1/AnimMontage/mutant_punch_Montage.mutant_punch_Montage"))

(event `PlaySkillAnim_Req`
  ;[1 1 1] PlaySkillAnim
  (`self.PlaySkillAnim_Multicast`))

(event `Attack_Skill`
  ;[1 1 1] Skill
)

(event `PlaySkillAnim_Multicast`
  ;[1 1 1] PlaySkillAnim
  (bind _returnvalue (`self.PlayAnimMontage` "/Game/Enemy/Boss/Boss1/AnimMontage/mutant_flexing_muscles_Montage.mutant_flexing_muscles_Montage"))
  (`KismetSystemLibrary.Delay` _returnvalue)
  (`self.PlayAnimMontage` "/Game/Enemy/Boss/Boss1/AnimMontage/mutant_swiping_Montage.mutant_swiping_Montage"))

(event `Attack`
  ;[1 1 1] Attack
)

(event `self.Capsule1.OnComponentBeginOverlap`
  (params (OverlappedComponent :type "PrimitiveComponent Object Reference") (OtherActor :type "Actor Object Reference") (OtherComp :type "PrimitiveComponent Object Reference") (OtherBodyIndex :type Integer) (bFromSweep :type Boolean) (SweepResult :type "HitResult Structure (by ref)"))
  ;[1 1 1] AnyDamage Overlap
  (`|ExecutionSequence`
    (:`then_0`
      (bind _asbp_player_base (cast `/Game/Characters/BP_PlayerBase` OtherActor))
      (if (`self.ActorHasTag` _asbp_player_base "Player")
        (`self.ApplyAnyDamagePlayer_Req` _asbp_player_base (`self.SkillDamage`))
        (bind _returnvalue (`self.K2_GetActorLocation` _asbp_player_base))
        (`GameplayStatics.SpawnEmitterAtLocation` "/Game/WeaponEffects/P_body_bullet_impact.P_body_bullet_impact" _returnvalue (struct) (2.0 2.0 2.0))
        (`self.ShowAttackEffect_Req` true _returnvalue)))
    (:`then_1`
      (bind _asbp_nexus (cast `/Game/Nexus/BP_Nexus` OtherActor))
      (`self.ApplyAnyDamageNexus_Req` _asbp_nexus (`self.SkillDamage`))
      (bind _returnvalue_2 (`self.K2_GetActorLocation` _asbp_nexus))
      (`GameplayStatics.SpawnEmitterAtLocation` "/Game/WeaponEffects/P_body_bullet_impact.P_body_bullet_impact" _returnvalue_2 (struct) (2.0 2.0 2.0))
      (`self.ShowAttackEffect_Req` false _returnvalue_2))))

(event `self.Sphere.OnComponentBeginOverlap`
  (params (OverlappedComponent :type "PrimitiveComponent Object Reference") (OtherActor :type "Actor Object Reference") (OtherComp :type "PrimitiveComponent Object Reference") (OtherBodyIndex :type Integer) (bFromSweep :type Boolean) (SweepResult :type "HitResult Structure (by ref)"))
  ;[1 1 1] AnyDamage Overlap
  (`|ExecutionSequence`
    (:`then_0`
      (bind _asbp_player_base (cast `/Game/Characters/BP_PlayerBase` OtherActor))
      (if (`self.ActorHasTag` _asbp_player_base "Player")
        (`self.ApplyAnyDamagePlayer_Req` _asbp_player_base (`self.Damage`))
        (bind _returnvalue (`self.K2_GetActorLocation` _asbp_player_base))
        (`GameplayStatics.SpawnEmitterAtLocation` "/Game/WeaponEffects/P_body_bullet_impact.P_body_bullet_impact" _returnvalue (struct) (2.0 2.0 2.0))
        (`self.ShowAttackEffect_Req` true _returnvalue)))
    (:`then_1`
      (bind _asbp_nexus (cast `/Game/Nexus/BP_Nexus` OtherActor))
      (`self.ApplyAnyDamageNexus_Req` _asbp_nexus (`self.Damage`))
      (bind _returnvalue_2 (`self.K2_GetActorLocation` _asbp_nexus))
      (`GameplayStatics.SpawnEmitterAtLocation` "/Game/WeaponEffects/P_body_bullet_impact.P_body_bullet_impact" _returnvalue_2 (struct) (2.0 2.0 2.0))
      (`self.ShowAttackEffect_Req` false _returnvalue_2))))

(fn `OnRep_Death`
  (`|ExecutionSequence`
    (:`then_0`
      (`GameplayStatics.PlaySoundAtLocation` "/Game/Sounds_StrategyGame/Characters/CrowdTaunts/Sound_Boss_Death.Sound_Boss_Death" (`self.K2_GetActorLocation`))
      (set `CharacterMovementComponent.MaxWalkSpeed` 0.0 (`self.CharacterMovement`))
      (set `/Game/GameModes/Zombie/BP_ZombieGM.PlayingState` "NewEnumerator2" (`self.GameMode`)))
    (:`then_1`
      (`/Game/GameModes/Zombie/BP_ZombiePC.DecreaseZombie` (`self.PlayerController`)))))

(fn `OnRep_IsAttacking`
  (if (`self.IsAttacking`)
    (set `CharacterMovementComponent.MaxWalkSpeed` 0.0 (`self.CharacterMovement`))
    (set `self.AttackTime` 3.0)))

(fn `OnRep_MainTarget`
  (`self.SetActorTickEnabled` true))

(fn `SaveDisAndDir`
  (bind _maintarget (`self.MainTarget`))
  (bind _returnvalue (- (`self.K2_GetActorLocation` _maintarget) (`self.K2_GetActorLocation`)))
  (`/Engine/EditorBlueprintResources/StandardMacros.IsValid` _maintarget
    (:`Is Valid`
      _)
    (:`Is Not Valid`
      (bind _asbp_zombie_gm (cast `/Game/GameModes/Zombie/BP_ZombieGM` (`GameplayStatics.GetGameMode`)))
      (set `self.MainTarget` (`/Game/GameModes/Zombie/BP_ZombieGM.MainTarget` _asbp_zombie_gm))))
  (set `self.DistancePlayerChar` (`KismetMathLibrary.VSize` _returnvalue))
  (set `self.DirToPlayerChar` (`KismetMathLibrary.Normal` _returnvalue)))

(fn `UserConstructionScript`)